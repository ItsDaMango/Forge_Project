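; One-shot trigger volume that adds the player character's UI widget to the viewport when the player first enters it.
; The overlap marks it activated, disables collision and saves its state by ID in the game instance's SavedGame.
; It binds to the game instance's OnGameLoaded event to restore that state, so an activated trigger stays spent after loading.
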(event `self.ReceiveBeginPlay`
  (bind _asbp_game_instance (cast `/Game/MyContent/Core/BP_GameInstance` (`GameplayStatics.GetGameInstance`)))
  (bind _output_get (set `self.GameInstanceRef` _asbp_game_instance))
  (add `/Game/MyContent/Core/BP_GameInstance.OnGameLoaded` _output_get (`|CreateDelegate` :!event `OnGameLoaded`)))

(event `self.Trigger_Zone.OnComponentBeginOverlap`
  (params (OverlappedComponent :type "PrimitiveComponent Object Reference") (OtherActor :type "Actor Object Reference") (OtherComp :type "PrimitiveComponent Object Reference") (OtherBodyIndex :type Integer) (bFromSweep :type Boolean) (SweepResult :type "HitResult Structure (by ref)"))
  (if (not (`self.Activated`))
    (bind _asbp_player_character (cast `/Game/MyContent/Player/BP_PlayerCharacter` OtherActor))
    (`/Engine/EditorBlueprintResources/StandardMacros.IsValid` _asbp_player_character
      (:`Is Valid`
        (`UserWidget.AddToViewport` (`/Game/MyContent/Player/BP_PlayerCharacter.UIRef` _asbp_player_character) 5)
        (`PrimitiveComponent.SetCollisionEnabled` (`self.Trigger_Zone`) "NoCollision")
        (set `self.Activated` true)
        (`self.CreateSaveData`)))))

(fn `CreateSaveData`
  (bind _triggerboxes (`/Game/MyContent/SaveGame/BP_SaveGame.TriggerBoxes` (`/Game/MyContent/Core/BP_GameInstance.SavedGame` (`self.GameInstanceRef`))))
  (if (not (`KismetArrayLibrary.Array_Contains` _triggerboxes (make `/Game/MyContent/SaveGame/S_SpawnerTriggerBox` false (`self.ID`))))
    (`KismetArrayLibrary.Array_Add` _triggerboxes (make `/Game/MyContent/SaveGame/S_SpawnerTriggerBox` (`self.Activated`) (`self.ID`)))
    (`/Game/MyContent/Core/BP_GameInstance.CreateSaveGame` (`self.GameInstanceRef`))))

(fn `OnGameLoaded`
  (bind _gameinstanceref (`self.GameInstanceRef`))
  (bind _debug (`/Game/MyContent/Core/BP_GameInstance.Debug` _gameinstanceref))
  (for _array_element (`/Game/MyContent/SaveGame/BP_SaveGame.TriggerBoxes` (`/Game/MyContent/Core/BP_GameInstance.SavedGame` _gameinstanceref))
    (bind (_shouldactivate _id) (break `/Game/MyContent/SaveGame/S_SpawnerTriggerBox` _array_element))
    (if (== (`self.ID`) _id)
      (set `self.Activated` _shouldactivate)
      (else
        (`KismetSystemLibrary.PrintString` "BP_Trigger: Not Saved" _debug _debug (struct :`R` 0.014539 :`G` 1.0 :`B` 0.439967 :`A` 1.0))))))

(fn `UserConstructionScript`)