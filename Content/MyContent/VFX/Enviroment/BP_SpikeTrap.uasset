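; Spike trap actor that deals fixed damage to any actor overlapping its collision, with a timeline that moves the spikes vertically.
; If enabled at BeginPlay, it sets a looping timer using ActivateTime, or a random interval when that is not positive.
; OnInteract only sets the enabled flag without starting the timer, and IsInteractable returns false.
; Damage is independent of the animation, as the collision toggles are unwired.
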(event `self.ReceiveBeginPlay`
  (if (`self.TrapEnabled`)
    (`KismetSystemLibrary.K2_SetTimerDelegate` (`|CreateDelegate` :!event `PlayTrapAnim`) (select `bool` (> (`self.ActivateTime`) 0.0) :`false` (`KismetMathLibrary.RandomFloatInRange` 2.0 12.0) :`true` (`self.ActivateTime`) :!type "Float (single-precision)") true)))

(event `EnableTrap`
  (set `self.TrapEnabled` true))

(event `PlayTrapAnim`
  (bind (_direction _newtrack_0) (`Timeline|Timeline`)
    (:`Update`
      (`SceneComponent.K2_SetRelativeLocation` (`self.Spikes`) (`KismetMathLibrary.MakeVector` 0.0 0.0 (`KismetMathLibrary.Lerp` -300.0 0.0 _newtrack_0)) false false))))

(event `self.DamageCollision.OnComponentBeginOverlap`
  (params (OverlappedComponent :type "PrimitiveComponent Object Reference") (OtherActor :type "Actor Object Reference") (OtherComp :type "PrimitiveComponent Object Reference") (OtherBodyIndex :type Integer) (bFromSweep :type Boolean) (SweepResult :type "HitResult Structure (by ref)"))
  (`GameplayStatics.ApplyDamage` OtherActor 10.0))

(event `/Game/MyContent/Interface/BPI_InteractInterface.OnInteract`
  (params (`Interacting Actor` :type "Actor Object Reference") (IsHolding :type Boolean))
  (`self.EnableTrap`))

(fn `IsInteractable`
  (returns (Interactable :type Boolean))
  (return false))

(fn `UserConstructionScript`)