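; BP_I_ServerButton is a hold-to-complete interactible with a red glowing dynamic material and a timeline-animated text prompt.
; Holding it runs a looping one-second countdown shown on the text, and the first hold also starts the linked TurnOffSpawners spawning.
; Releasing resets the countdown.
; At zero it messages linked Interactibles, stops those spawners and disables itself, hiding the prompt and glow.
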(event `self.ReceiveBeginPlay`
  (`parent.ReceiveBeginPlay`)
  (`self.InteractText`)
  (set `self.CountDown` (`self.TimeToCountDownFrom`)))

(event `/Game/MyContent/Interface/BPI_InteractInterface.OnInteract`
  (params (`Interacting Actor` :type "Actor Object Reference") (IsHolding :type Boolean))
  (if (`self.Active`)
    (if IsHolding
      (`/Engine/EditorBlueprintResources/StandardMacros.DoOnce` false :!label _label
        (:`Completed`
          (`self.StopInteractText`)
          (`SceneComponent.SetVisibility` (`self.Txt`) true false)
          (bind _output_get (set `self.CountDown` (- (`self.CountDown`) 1)))
          (`TextRenderComponent.K2_SetText` (`self.Txt`) (`|FormatText` "Hold '{time}'" _output_get))
          (`KismetSystemLibrary.K2_SetTimerDelegate` (`|CreateDelegate` :!event `CountdownTimer`) 1.0 true)
          (`/Engine/EditorBlueprintResources/StandardMacros.DoOnce` false
            (:`Completed`
              (for _array_element (`self.TurnOffSpawners`)
                (set `/Game/MyContent/Enemies/Spawning/BP_SpawnPoint.Activated` true _array_element)
                (set `/Game/MyContent/Enemies/Spawning/BP_SpawnPoint.CanBeActivated` true _array_element)
                (`KismetSystemLibrary.K2_SetTimer` _array_element "Spawning" 0.2 true))))))
      (else
        (`self.ResetTimer`)
        (goto _label :!via `Reset`)))))

(event `StopInteractText`
  (bind _returnvalue (`SceneComponent.K2_GetComponentLocation` (`self.Scene`)))
  (bind (_direction _newtrack_0) (`Timeline|TL_TextMovement` :!via `Stop` :!label _label_2)
    (:`Update`
      (`TextRenderComponent.SetTextRenderColor` (`self.Txt`) (`KismetMathLibrary.Conv_LinearColorToColor` (`KismetMathLibrary.LinearColorLerp` (struct :`R` 0.640625 :`G` 0.640625 :`B` 0.640625 :`A` 0.26087) (struct :`R` 27.560877 :`G` 29.582357 :`B` 30.0 :`A` 1.0) _newtrack_0)))
      (`SceneComponent.K2_SetWorldLocation` (`self.Txt`) (`KismetMathLibrary.VLerp` (+ _returnvalue (0.0 0.0 0.0)) (+ _returnvalue (0.0 0.0 25.0)) _newtrack_0) false false))
    (:`Finished`
      (`self.InteractText`))))

(event `InteractText`
  (`TextRenderComponent.K2_SetText` (`self.Txt`) (`|FormatText` "Press E To Interact"))
  (goto _label_2 :!via `PlayFromStart`))

(fn `CountdownTimer`
  (bind _output_get (set `self.CountDown` (`KismetMathLibrary.Max` (- (`self.CountDown`) 1))))
  (`TextRenderComponent.K2_SetText` (`self.Txt`) (`|FormatText` "Hold '{time}'" _output_get))
  ; WHATEVER U WANT TO HAPPEN WHEN IT HITS 0 GOES HERE
  (if (<= (`self.CountDown`) 0)
    (for _array_element (`self.Interactibles`)
      (message `/Game/MyContent/Interface/BPI_InteractInterface.OnInteract` _array_element null false))
    (for _array_element_2 (`self.TurnOffSpawners`)
      (`/Game/MyContent/Enemies/Spawning/BP_SpawnPoint.StopSpawning` _array_element_2))
    (`self.DisableSelf`)))

(fn `DisableSelf`
  (set `self.Active` false)
  (`self.StopInteractText`)
  (`SceneComponent.SetVisibility` (`self.Txt`) false false)
  (`MaterialInstanceDynamic.SetScalarParameterValue` (`self.MI_DynamicMaterial`) "Strength" 0.0))

(fn `IsInteractable`
  (returns (Interactable :type Boolean))
  (return true))

(fn `ResetTimer`
  (`KismetSystemLibrary.K2_ClearTimer` null "CountdownTimer")
  (set `self.CountDown` (`self.TimeToCountDownFrom`))
  (`self.InteractText`))

(fn `UserConstructionScript`
  (`parent.UserConstructionScript`)
  (bind _returnvalue (`PrimitiveComponent.CreateDynamicMaterialInstance` (`self.StaticMesh`) 0 null "None"))
  (bind _output_get (set `self.MI_DynamicMaterial` _returnvalue))
  (`MaterialInstanceDynamic.SetVectorParameterValue` _output_get "Colour" (struct :`R` 1.0 :`G` 0.028372 :`A` 1.0))
  (`MaterialInstanceDynamic.SetScalarParameterValue` _output_get "Strength" 40.0))