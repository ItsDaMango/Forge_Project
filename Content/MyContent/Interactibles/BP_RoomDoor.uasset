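; BP_RoomDoor is an interactable, key-gated room door that swings open once.
; OnInteract decrements the required key count and opens at zero; overlapping the closed, keyless door sends an OnInteract message to the player.
; Opening turns the lights green, optionally switching them off, while a timeline feeds RInterpTo as DeltaTime, rotating relative to current yaw.
; Reverse flips swing direction and selects visible arrow, light and exit sign in construction.
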(event `self.ReceiveBeginPlay`
  (`parent.ReceiveBeginPlay`))

(event `OpenDoor`
  (bind (_returnvalue_roll _returnvalue_pitch _returnvalue_yaw) (`KismetMathLibrary.BreakRotator` (`SceneComponent.K2_GetComponentRotation` (`self.Scene`))))
  (if (not (not (`self.NoLightOnOpen`)))
    (`LightComponent.SetIntensity` (`self.LightReverse`) 0.0)
    (`LightComponent.SetIntensity` (`self.RectLight`) 0.0))
  (`LightComponent.SetLightColor` (`self.RectLight`) (struct :`R` 0.142705 :`G` 1.0 :`B` 0.00914 :`A` 1.0) true)
  (`LightComponent.SetLightColor` (`self.LightReverse`) (struct :`R` 0.142705 :`G` 1.0 :`B` 0.00914 :`A` 1.0) true)
  (bind (_direction _alpha) (`Timeline|TL_Door` :!via `PlayFromStart`)
    (:`Update`
      (`SceneComponent.K2_SetWorldRotation` (`self.Scene`) (`KismetMathLibrary.RInterpTo` (`SceneComponent.K2_GetComponentRotation` (`self.Scene`)) (`KismetMathLibrary.MakeRotator` 0.0 0.0 (+ _returnvalue_yaw (select `bool` (`self.Reverse`) :`false` (* (`self.OpenAmount`) -1.0) :`true` (`self.OpenAmount`)))) _alpha 10.0) false false))))

(event `self.Collision.OnComponentBeginOverlap`
  (params (OverlappedComponent :type "PrimitiveComponent Object Reference") (OtherActor :type "Actor Object Reference") (OtherComp :type "PrimitiveComponent Object Reference") (OtherBodyIndex :type Integer) (bFromSweep :type Boolean) (SweepResult :type "HitResult Structure (by ref)"))
  (if (and (<= (`self.KeysNeededToOpen`) 0) (not (`self.Open`)))
    (bind _asbp_player_character (cast `/Game/MyContent/Player/BP_PlayerCharacter` OtherActor))
    (message `/Game/MyContent/Interface/BPI_InteractInterface.OnInteract` self _asbp_player_character)))

(event `/Game/MyContent/Interface/BPI_InteractInterface.OnInteract`
  (params (`Interacting Actor` :type "Actor Object Reference"))
  (set `self.KeysNeededToOpen` (`KismetMathLibrary.Max` (- (`self.KeysNeededToOpen`) 1)))
  (if (and (<= (`self.KeysNeededToOpen`) 0) (not (`self.Open`)))
    (set `self.Open` true)
    (`self.OpenDoor`)))

(fn `IsInteractable`
  (returns (Interactable :type Boolean))
  (return true))

(fn `UserConstructionScript`
  (`parent.UserConstructionScript`)
  (`SceneComponent.SetVisibility` (`self.DirectionReverse`) (`self.Reverse`) false)
  (`SceneComponent.SetVisibility` (`self.LightReverse`) (`self.Reverse`) false)
  (`SceneComponent.SetVisibility` (`self.ExitReverse`) (`self.Reverse`) false)
  (`SceneComponent.SetVisibility` (`self.Direction`) (not (`self.Reverse`)) false)
  (`SceneComponent.SetVisibility` (`self.RectLight`) (not (`self.Reverse`)) false)
  (`SceneComponent.SetVisibility` (`self.ExitSign`) (not (`self.Reverse`)) false))