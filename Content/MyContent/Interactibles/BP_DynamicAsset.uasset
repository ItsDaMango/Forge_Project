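; BP_DynamicAsset is a configurable interactible actor that plays an effect and a sound when used.
; The construction script applies the chosen mesh and multiplies the mesh transform scale and sphere collision radius by AssetScale.
; OnInteract spawns an attached Niagara system slightly above the mesh and a sound at the actor's location.
; A separate Destroy function removes the actor and is not called within this Blueprint.
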(event `self.ReceiveBeginPlay`
  (`parent.ReceiveBeginPlay`))

(event `/Game/MyContent/Interface/BPI_InteractInterface.OnInteract`
  (params (`Interacting Actor` :type "Actor Object Reference") (IsHolding :type Boolean))
  (`NiagaraFunctionLibrary.SpawnSystemAttached` (`self.SystemEffect`) (`self.Mesh`) "None" (+ (`SceneComponent.K2_GetComponentLocation` (`self.Mesh`)) (0.0 0.0 30.0)) (`SceneComponent.K2_GetComponentRotation` (`self.MeshTransform`)) "KeepWorldPosition" false true "AutoRelease")
  (`GameplayStatics.SpawnSoundAtLocation` (`self.SoundEffect`) (`self.K2_GetActorLocation`) (struct) 0.8 1.0 0.0 null null))

(fn `Destroy`
  (`self.K2_DestroyActor`))

(fn `UserConstructionScript`
  (bind _collision (`self.Collision`))
  (bind (_returnvalue_location _returnvalue_rotation _returnvalue_scale) (`KismetMathLibrary.BreakTransform` (`SceneComponent.K2_GetComponentToWorld` (`self.MeshTransform`))))
  (`parent.UserConstructionScript`)
  (`StaticMeshComponent.SetStaticMesh` (`self.Mesh`) (`self.MainMesh`))
  (`SceneComponent.K2_SetWorldTransform` (`self.MeshTransform`) (`KismetMathLibrary.MakeTransform` _returnvalue_location _returnvalue_rotation (* _returnvalue_scale (`self.AssetScale`))) false false)
  (`SphereComponent.SetSphereRadius` _collision (* (`SphereComponent.SphereRadius` _collision) (`self.AssetScale`)) true))