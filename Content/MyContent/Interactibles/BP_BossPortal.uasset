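; BP_BossPortal is an interactible portal that opens after enough key interactions and moves the game to the next level or end screen.
; Each interaction decrements the key count; at zero, coloured Niagara effects activate.
; Player overlap on the open portal clears saved locations and saves the target level.
; A "MENU" tag shows a paused end screen; otherwise, a save-completion callback removes players and swaps streamed levels.
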(event `self.ReceiveBeginPlay`
  (`parent.ReceiveBeginPlay`)
  (bind _asbp_game_instance (cast `/Game/MyContent/Core/BP_GameInstance` (`GameplayStatics.GetGameInstance`)))
  (bind _output_get (set `self.GameInstanceRef` _asbp_game_instance))
  (add `/Game/MyContent/Core/BP_GameInstance.OnGameSaved` _output_get (`|CreateDelegate` :!event `TryLoadNewLevel`))
  (bind _asbp_gm_main (cast `/Game/MyContent/Core/BP_GM_Main` (`GameplayStatics.GetGameMode`)))
  (set `self.GameModeRef` _asbp_gm_main)
  (set `self.CanTryStreamLevel` false))

(event `/Game/MyContent/Interface/BPI_InteractInterface.OnInteract`
  (params (`Interacting Actor` :type "Actor Object Reference") (IsHolding :type Boolean))
  (bind _portalcolour_ (`self.PortalColour `))
  (set `self.Keys Needed to Open` (`KismetMathLibrary.Clamp` (- (`self.Keys Needed to Open`) 1) 0 (`self.Keys Needed to Open`)))
  (if (<= (`self.Keys Needed to Open`) 0)
    (`ActorComponent.Activate` (`self.ActivePortal`) true)
    (`ActorComponent.Activate` (`self.NS_BlowingParticle`) true)
    (`ActorComponent.Deactivate` (`self.Niagara`))
    (`NiagaraComponent.SetVariableLinearColor` (`self.NS_BlowingParticle`) "P_Colour" _portalcolour_)
    (`NiagaraComponent.SetVariableLinearColor` (`self.ActivePortal`) "P_Colour" _portalcolour_)))

(event `self.Collision.OnComponentBeginOverlap`
  (params (OverlappedComponent :type "PrimitiveComponent Object Reference") (OtherActor :type "Actor Object Reference") (OtherComp :type "PrimitiveComponent Object Reference") (OtherBodyIndex :type Integer) (bFromSweep :type Boolean) (SweepResult :type "HitResult Structure (by ref)"))
  (bind _worlddata_playerlocation (break `/Game/MyContent/SaveGame/S_WorldData` (`/Game/MyContent/SaveGame/BP_SaveGame.WorldData` (`/Game/MyContent/Core/BP_GameInstance.SavedGame` (`self.GameInstanceRef`)))))
  (cast `/Game/MyContent/Player/BP_PlayerCharacter` OtherActor)
  (if (<= (`self.Keys Needed to Open`) 0)
    (set `self.CanTryStreamLevel` true)
    (`KismetArrayLibrary.Array_Clear` _worlddata_playerlocation)
    (`self.CreateSaveData`)
    (if (== (`self.Tag`) "MENU")
      (bind _outactors (`GameplayStatics.GetAllActorsOfClass` "/Game/MyContent/Player/BP_PlayerCharacter.BP_PlayerCharacter_C"))
      (for _array_element _outactors
        (`/Game/MyContent/Player/BP_PlayerCharacter.RemoveInput` _array_element false (`|MakeArray` "/Game/MyContent/Player/Input/IMC_Core.IMC_Core" "/Game/MyContent/Player/Input/IMC_Movement.IMC_Movement" "/Game/MyContent/Player/Input/IMC_Combat.IMC_Combat" :!type "InputMappingContext Object Reference")))
      (bind _returnvalue (`|CreateWidget` "/Game/MyContent/Menus/EndGameMenu/BP_UI_EndScreen.BP_UI_EndScreen_C"))
      (`UserWidget.AddToViewport` _returnvalue 0)
      (`GameplayStatics.SetGamePaused` true)
      (`Widget.RemoveFromParent` (`/Game/MyContent/Core/BP_GM_Main.GM_HUD` (`self.GameModeRef`))))))

(event `TryLoadNewLevel`
  (params (IsQuiting :type Boolean))
  (if (!= (`self.Tag`) "MENU")
    (if (`self.CanTryStreamLevel`)
      (`self.RemovePlayers`)
      (`/Game/MyContent/Core/BP_GM_Main.StreamLevel` (`self.GameModeRef`) "None" "None")
      (`/Game/MyContent/Core/BP_GM_Main.UnstreamLevels` :`self` (`self.GameModeRef`)))))

(fn `CreateSaveData`
  (set `/Game/MyContent/SaveGame/BP_SaveGame.CurrentLevel` (make `/Game/MyContent/SaveGame/S_LevelData` (`self.Level Name`) (`self.Tag`) (`self.Unload Levels`)) (`/Game/MyContent/Core/BP_GameInstance.SavedGame` (`self.GameInstanceRef`)))
  (`/Game/MyContent/Core/BP_GameInstance.CreateSaveGame` (`self.GameInstanceRef`)))

(fn `RemovePlayers`
  (bind _outactors (`GameplayStatics.GetAllActorsOfClass` "/Game/MyContent/Player/BP_PlayerCharacter.BP_PlayerCharacter_C"))
  (for _array_element _outactors
    (if (`KismetSystemLibrary.IsValid` _array_element)
      (`self.K2_DestroyActor` _array_element)))
  (bind _outactors_2 (`GameplayStatics.GetAllActorsOfClass` "/Game/MyContent/Player/BP_PlayerController.BP_PlayerController_C"))
  (for _array_element_2 _outactors_2
    (`GameplayStatics.RemovePlayer` _array_element_2 true))
  (set `/Game/MyContent/Core/BP_GM_Main.PlayerIndex` 0 (`self.GameModeRef`)))

(fn `UserConstructionScript`
  (`parent.UserConstructionScript`))