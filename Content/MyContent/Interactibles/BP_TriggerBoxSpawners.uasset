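; BP_TriggerBoxSpawners is a trigger box that starts its linked Spawners when BP_PlayerCharacter overlaps it, gated by a DoOnce.
; Activation flags each spawner and starts a looping timer on its Spawning function, calling CreateSaveData to store the box's ID and Activated state through BP_GameInstance.
; On game load, a bound handler matches the saved ID and, if flagged active, replays the same activation after a short delay.
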(event `self.ReceiveBeginPlay`
  (`parent.ReceiveBeginPlay`)
  (bind _asbp_game_instance (cast `/Game/MyContent/Core/BP_GameInstance` (`GameplayStatics.GetGameInstance`)))
  (bind _output_get (set `self.GameInstanceRef` _asbp_game_instance))
  (add `/Game/MyContent/Core/BP_GameInstance.OnGameLoaded` _output_get (`|CreateDelegate` :!event `OnGameLoaded`)))

(event `ActivateFromLoad`
  (bind _spawners (`self.Spawners`))
  (`KismetSystemLibrary.Delay` 0.2)
  (if (`KismetArrayLibrary.Array_IsNotEmpty` _spawners) :!label _label
    (for _array_element _spawners
      (set `/Game/MyContent/Enemies/Spawning/BP_SpawnPoint.Activated` true _array_element)
      (`KismetSystemLibrary.K2_SetTimer` _array_element "Spawning" 0.2 true)
      (`self.CreateSaveData`))))

(event `self.TriggerCollision.OnComponentBeginOverlap`
  (params (OverlappedComponent :type "PrimitiveComponent Object Reference") (OtherActor :type "Actor Object Reference") (OtherComp :type "PrimitiveComponent Object Reference") (OtherBodyIndex :type Integer) (bFromSweep :type Boolean) (SweepResult :type "HitResult Structure (by ref)"))
  (`/Engine/EditorBlueprintResources/StandardMacros.DoOnce` false
    (:`Completed`
      (cast `/Game/MyContent/Player/BP_PlayerCharacter` OtherActor)
      (goto _label))))

(event `/Game/MyContent/Interface/BPI_InteractInterface.OnInteract`
  (params (`Interacting Actor` :type "Actor Object Reference") (IsHolding :type Boolean)))

(fn `CreateSaveData`
  (bind _triggerboxes (`/Game/MyContent/SaveGame/BP_SaveGame.TriggerBoxes` (`/Game/MyContent/Core/BP_GameInstance.SavedGame` (`self.GameInstanceRef`))))
  (if (not (`KismetArrayLibrary.Array_Contains` _triggerboxes (make `/Game/MyContent/SaveGame/S_SpawnerTriggerBox` false (`self.ID`))))
    (`KismetArrayLibrary.Array_Add` _triggerboxes (make `/Game/MyContent/SaveGame/S_SpawnerTriggerBox` (`self.Activated`) (`self.ID`)))
    (`/Game/MyContent/Core/BP_GameInstance.CreateSaveGame` (`self.GameInstanceRef`))))

(fn `OnGameLoaded`
  (for _array_element (`/Game/MyContent/SaveGame/BP_SaveGame.TriggerBoxes` (`/Game/MyContent/Core/BP_GameInstance.SavedGame` (`self.GameInstanceRef`)))
    (bind (_shouldactivate _id) (break `/Game/MyContent/SaveGame/S_SpawnerTriggerBox` _array_element))
    (if (== (`self.ID`) _id)
      (set `self.Activated` _shouldactivate)
      (if (`self.Activated`)
        (`self.ActivateFromLoad`)))))

(fn `UserConstructionScript`
  (`parent.UserConstructionScript`))