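; BP_Collision is an interactible actor with a Wall component whose appearance switches between entries in a Materials array.
; BeginPlay creates dynamic instances from each entry, then applies the first array material to the wall.
; SetMaterial applies a material by slot index, and SetDefaultMaterial restores the first.
; ResetMaterial starts a short looping event timer, while SetDefaultMaterial attempts to clear a timer by its own function name.
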(event `self.ReceiveBeginPlay`
  (bind _materials (`self.Materials`))
  (for _array_element _materials
    (`PrimitiveComponent.CreateDynamicMaterialInstance` (`self.Wall`) 0 _array_element "None"))
  (`PrimitiveComponent.SetMaterial` (`self.Wall`) 0 (`|GetArrayItem` _materials)))

(fn `ResetMaterial`
  (`KismetSystemLibrary.K2_SetTimerDelegate` (`|CreateDelegate` :!event `SetDefaultMaterial`) 0.3 true))

(fn `SetDefaultMaterial`
  (`self.SetMaterial` 0)
  (`KismetSystemLibrary.K2_ClearTimer` null "SetDefaultMaterial"))

(fn `SetMaterial`
  (params (MaterialSlot :type Integer))
  (`PrimitiveComponent.SetMaterial` (`self.Wall`) 0 (`|GetArrayItem` (`self.Materials`) MaterialSlot)))

(fn `UserConstructionScript`)