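; BP_WeaponSpear is a spear weapon Blueprint with projectile movement and a damage collision component.
; On BeginPlay it runs the parent logic, sets the projectile's initial speed and makes the damage collision query-only.
; It adds no overlap, tick or construction behavior of its own, leaving anything further to its parent class.
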(event `self.ReceiveBeginPlay`
  (`parent.ReceiveBeginPlay`)
  (set `ProjectileMovementComponent.InitialSpeed` 1000.0 (`self.ProjectileMovement`))
  (`PrimitiveComponent.SetCollisionEnabled` (`self.DamageCollision`) "QueryOnly"))

(fn `UserConstructionScript`
  (`parent.UserConstructionScript`))