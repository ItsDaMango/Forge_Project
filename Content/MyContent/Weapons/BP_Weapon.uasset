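; BP_Weapon is a weapon actor that applies damage to actors overlapping its DamageCollision, excluding its owner and ignored classes.
; ActivateDamage and DeactivateDamage toggle that collision between query-only and disabled.
; IsIgnoredClass matches when a ClassToIgnore entry is a child of the hit actor's class, so the check runs from list entry to actor.
; Niagara attack and portal effect spawns exist but are disconnected.
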(event `self.DamageCollision.OnComponentBeginOverlap`
  (params (OverlappedComponent :type "PrimitiveComponent Object Reference") (OtherActor :type "Actor Object Reference") (OtherComp :type "PrimitiveComponent Object Reference") (OtherBodyIndex :type Integer) (bFromSweep :type Boolean) (SweepResult :type "HitResult Structure (by ref)"))
  (bind _output_get (set `self.HitActor` OtherActor))
  (if (and (!= OtherActor (`self.GetOwner`)) (not (`self.IsIgnoredClass` OtherActor)))
    (`GameplayStatics.ApplyDamage` _output_get (`self.Damage`) null (`self.GetOwner`))))

(fn `ActivateDamage`
  (`PrimitiveComponent.SetCollisionEnabled` (`self.DamageCollision`) "QueryOnly"))

(fn `DeactivateDamage`
  (`PrimitiveComponent.SetCollisionEnabled` (`self.DamageCollision`) "NoCollision"))

(fn `IsIgnoredClass`
  (params (TestActor :type "Actor Object Reference"))
  (returns (IsIgnoredClass :type Boolean))
  (for _array_element (`self.ClassToIgnore`)
    (if (`KismetMathLibrary.ClassIsChildOf` _array_element (`GameplayStatics.GetObjectClass` TestActor))
      (return true)))
  (return false))

(fn `UserConstructionScript`)