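; Character stats component that holds skill points and energy values and broadcasts their changes.
; Setters floor values at zero, with no clamp to the maximum, then call the matching changed dispatcher.
; AddSkillPoints routes through SetSkillPoints and also broadcasts the added amount.
; SetEnergy writes MaxEnergy just as SetMaxEnergy does, so no function here sets a separate current energy value.
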(fn `AddSkillPoints`
  (params (Amount :type Integer))
  (`self.SetSkillPoints` (+ (`self.SkillPoints`) Amount))
  (`self.OnSkillPointAdded` (`local.Amount`)))

(fn `SetEnergy`
  (params (MaxEnergy :type "Float (double-precision)"))
  (set `self.MaxEnergy` (`KismetMathLibrary.FMax` MaxEnergy))
  (`self.OnEnergyChanged`))

(fn `SetMaxEnergy`
  (params (MaxEnergy :type "Float (double-precision)"))
  (set `self.MaxEnergy` (`KismetMathLibrary.FMax` MaxEnergy))
  (`self.OnEnergyChanged`))

(fn `SetMaxSkillPoints`
  (params (MaxSkillPoints :type Integer))
  (set `self.MaxSkillPoints` (`KismetMathLibrary.Max` MaxSkillPoints))
  (`self.OnSkillPointsChanged`))

(fn `SetSkillPoints`
  (params (SkillPoints :type Integer))
  (set `self.SkillPoints` (`KismetMathLibrary.Max` SkillPoints))
  (`self.OnSkillPointsChanged`))