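; Main game mode for local multiplayer: sets up players, HUD and pause menu, and loads the save game.
; BeginPlay shows a loading screen, streams in Lvl_Boss_01, spawns and possesses characters at "Boss"-tagged PlayerStarts, then unloads other levels.
; StreamLevel loads another level and teleports both players to tagged starts; OpenLevel repeats player setup at "player" starts.
; Helpers toggle pause and trigger random enemy voice cues; RespawnPlayer is empty.
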(event `OpenLevel`
  (bind _outactors (`GameplayStatics.GetAllActorsOfClassWithTag` "/Script/Engine.PlayerStart" "player"))
  (if (`KismetArrayLibrary.Array_IsNotEmpty` _outactors)
    (for (_array_element _array_index) _outactors
      (bind _output_get (set `self.PlayerIndex` _array_index))
      (bind _returnvalue (`GameplayStatics.CreatePlayer` _output_get))
      (if (< 0 (`self.PlayerIndex`))
        (bind _returnvalue_2 (`self.GetTransform` _array_element))
        (bind _returnvalue_3 (`|SpawnActorFromClass` "/Game/MyContent/Player/BP_PlayerCharacter.BP_PlayerCharacter_C" _returnvalue_2 "AdjustIfPossibleButAlwaysSpawn" "MultiplyWithRoot" null null))
        (set `/Game/MyContent/Player/BP_PlayerCharacter.PlayerIndex` 1 _returnvalue_3)
        (bind _asbp_player_controller (cast `/Game/MyContent/Player/BP_PlayerController` _returnvalue))
        (`Controller.Possess` _asbp_player_controller _returnvalue_3)
        (else
          (bind _returnvalue_4 (`|SpawnActorFromClass` "/Game/MyContent/Player/BP_PlayerCharacter.BP_PlayerCharacter_C" _returnvalue_2 "AdjustIfPossibleButAlwaysSpawn" "MultiplyWithRoot" null null))
          (set `/Game/MyContent/Player/BP_PlayerCharacter.PlayerIndex` 0 _returnvalue_4)
          (bind _asbp_player_controller_2 (cast `/Game/MyContent/Player/BP_PlayerController` (`GameplayStatics.GetPlayerController` 1)))
          (`Controller.Possess` _asbp_player_controller_2 _returnvalue_4))))
    (`self.CreateWidgets`)
    (bind _asbp_game_instance (cast `/Game/MyContent/Core/BP_GameInstance` (`GameplayStatics.GetGameInstance`)))
    (`/Game/MyContent/Core/BP_GameInstance.TryLoadGame` _asbp_game_instance)
    (`self.Initialise`)))

(event `self.ReceiveBeginPlay`
  (bind _returnvalue (`GameplayStatics.GetPlayerController` 0))
  (bind _debug (`self.Debug`))
  ;[0.15 0.002713 1.1e-05 0.5] Begin Play
  ;[0.09375 0.09375 0.09375 0.5] Add Loading Screen for seamless transition from menu
  (bind _returnvalue_2 (`|CreateWidget` "/Game/MyContent/Menus/MainMenu/BP_UI_LoadingScreen.BP_UI_LoadingScreen_C"))
  (bind _output_get (set `self.GM_LoadingScreen` _returnvalue_2))
  (`UserWidget.AddToViewport` _output_get 4)
  (`GameplayStatics.LoadStreamLevel` "Lvl_Boss_01" true)
  (set `self.PlayerIndex` 0)
  (bind _outactors (`GameplayStatics.GetAllActorsOfClassWithTag` "/Script/Engine.PlayerStart" "Boss"))
  (if (`KismetArrayLibrary.Array_IsNotEmpty` _outactors)
    (for (_array_element _array_index) _outactors
      (bind _output_get_2 (set `self.PlayerIndex` _array_index))
      (bind _returnvalue_3 (`GameplayStatics.CreatePlayer` _output_get_2))
      (if (< 0 (`self.PlayerIndex`))
        (bind _returnvalue_4 (`self.GetTransform` _array_element))
        (bind _returnvalue_5 (`|SpawnActorFromClass` "/Game/MyContent/Player/BP_PlayerCharacter.BP_PlayerCharacter_C" _returnvalue_4 "AlwaysSpawn" "MultiplyWithRoot" null null))
        (`KismetSystemLibrary.PrintString` "Player 2" _debug _debug (struct :`R` 1.0 :`G` 0.000304 :`B` 0.081785 :`A` 1.0) 3.0)
        (bind _asbp_player_controller (cast `/Game/MyContent/Player/BP_PlayerController` _returnvalue_3))
        (set `/Game/MyContent/Player/BP_PlayerController.PlayerIndex` 1 _asbp_player_controller)
        (`Controller.Possess` _asbp_player_controller _returnvalue_5)
        (else
          (bind _returnvalue_6 (`|SpawnActorFromClass` "/Game/MyContent/Player/BP_PlayerCharacter.BP_PlayerCharacter_C" _returnvalue_4 "AlwaysSpawn" "MultiplyWithRoot" null null))
          (`KismetSystemLibrary.PrintString` "Player 1" _debug _debug (struct :`R` 1.0 :`B` 0.429477 :`A` 1.0) 3.0)
          (bind _asbp_player_controller_2 (cast `/Game/MyContent/Player/BP_PlayerController` _returnvalue))
          (set `/Game/MyContent/Player/BP_PlayerController.PlayerIndex` 0 _asbp_player_controller_2)
          (`Controller.Possess` _returnvalue _returnvalue_6))))
    (`self.CreateWidgets`)
    (bind _asbp_game_instance (cast `/Game/MyContent/Core/BP_GameInstance` (`GameplayStatics.GetGameInstance`)))
    (`/Game/MyContent/Core/BP_GameInstance.TryLoadGame` _asbp_game_instance)
    (`self.UnstreamLevels` (`|MakeArray` "Lvl_Office_02" "Lvl_Boss_02" "Lvl_Office_01" :!type "Name"))
    ;[0.15 0.01048 0.01242 0.5] Initialise has to run somehwere here, preferably after most important stuff is called
    (`self.Initialise`)
    (`|ExecutionSequence`
      (:`then_0`
        ;[0.15 0.1341 0.05233 0.5] Get All enemies and play sound cue
        (`KismetSystemLibrary.K2_SetTimerDelegate` (`|CreateDelegate` :!event `GetAllAliveEnemies`) 15.0 true))
      (:`then_1`
        ;[0.03646 0.03646 0.03646 0.5] Remove Loading Screen After Delay
        (`KismetSystemLibrary.Delay` 0.8)
        (`Widget.RemoveFromParent` (`self.GM_LoadingScreen`))))
    (else
      (`KismetSystemLibrary.PrintString` "No player starts"))))

(event `self.ReceiveTick`
  (params (DeltaSeconds :type "Float (single-precision)")))

(event `UnstreamLevels`
  (params (Levels :type "Array of Name"))
  ;[0.15 0.0218 0.0132 0.5] Unstream Not Used Levels
  (for _array_element Levels
    (`GameplayStatics.UnloadStreamLevel` _array_element)))

(event `StreamLevel`
  (params (`Level ` :type Name) (Tag :type Name))
  ;[0.15 0.01472 0.01043 0.5] Stream In New level
  (`UserWidget.AddToViewport` (`self.GM_LoadingScreen`) 4)
  (`GameplayStatics.LoadStreamLevel` `Level ` true)
  (`self.SetPlayerLocations` Tag)
  (`Widget.RemoveFromParent` (`self.GM_LoadingScreen`)))

(fn `CreateWidgets`
  ; Menu? idk what this does honestly
  (bind _returnvalue (`|CreateWidget` "/Game/MyContent/Player/HUD/BP_UI_HUD.BP_UI_HUD_C"))
  (set `self.GM_Menu` _returnvalue)
  (bind _returnvalue_2 (`|CreateWidget` "/Game/MyContent/Player/HUD/BP_UI_HUD.BP_UI_HUD_C"))
  (set `self.GM_HUD` _returnvalue_2)
  (bind _returnvalue_3 (`|CreateWidget` "/Game/MyContent/Menus/PauseMenu/BP_UI_PauseMenu.BP_UI_PauseMenu_C"))
  (set `self.GM_PauseMenu` _returnvalue_3)
  (`UserWidget.AddToViewport` (`self.GM_HUD`) 1))

(fn `GetAllAliveEnemies`
  (if (and (not (`KismetArrayLibrary.Array_IsEmpty` (`self.EnemiesInLevel`))) (>= (`KismetArrayLibrary.Array_Length` (`self.EnemiesInLevel`)) 4))
    (for _ (range 4)
      (`/Game/MyContent/Enemies/BP_Enemy.SetVoiceCueTimer` (`KismetArrayLibrary.Array_Random` (`self.EnemiesInLevel`))))))

(fn `RespawnPlayer`)

(fn `SetPlayerLocations`
  (params (Tag :type Name))
  (bind _outactors (`GameplayStatics.GetAllActorsOfClassWithTag` "/Script/Engine.PlayerStart" Tag))
  (bind _outactors_2 (`GameplayStatics.GetAllActorsOfClass` "/Game/MyContent/Player/BP_PlayerCharacter.BP_PlayerCharacter_C"))
  (`self.K2_SetActorTransform` (`|GetArrayItem` _outactors_2) (`self.GetTransform` (`|GetArrayItem` _outactors)) false true)
  (`self.K2_SetActorTransform` (`|GetArrayItem` _outactors_2 1) (`self.GetTransform` (`|GetArrayItem` _outactors 1)) false true))

(fn `TogglePause`
  (`/Engine/EditorBlueprintResources/StandardMacros.FlipFlop`
    (:`A`
      (`UserWidget.AddToViewport` (`self.GM_PauseMenu`) 4)
      (`GameplayStatics.SetGamePaused` true)
      (`KismetSystemLibrary.PrintString` "on"))
    (:`B`
      (`Widget.RemoveFromParent` (`self.GM_PauseMenu`))
      (`GameplayStatics.SetGamePaused` false)
      (`KismetSystemLibrary.PrintString` "off"))))

(fn `UserConstructionScript`)