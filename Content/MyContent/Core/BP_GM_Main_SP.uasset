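; Main game mode (apparently single-player) that handles save-driven level streaming, player spawning and core UI.
; BeginPlay creates widgets and loads the save through BP_GameInstance, whose loaded callback streams in the saved level, spawns and possesses player 0, then unloads listed levels and destroys enemies.
; StreamLevel and UnstreamLevels ignore their level parameters, reading the save instead.
; Helpers toggle pause and settings, while teleport and death-screen functions still assume two players.
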(event `OpenLevel`
  (bind _outactors (`GameplayStatics.GetAllActorsOfClassWithTag` "/Script/Engine.PlayerStart" "Office"))
  (if (`KismetArrayLibrary.Array_IsNotEmpty` _outactors)
    (for (_array_element _array_index) _outactors
      (bind _output_get (set `self.PlayerIndex` _array_index))
      (`GameplayStatics.CreatePlayer` _output_get false)
      (if (< 0 (`self.PlayerIndex`))
        (bind _returnvalue (`self.GetTransform` _array_element))
        (bind _returnvalue_2 (`|SpawnActorFromClass` "/Game/MyContent/Player/BP_PlayerCharacter.BP_PlayerCharacter_C" _returnvalue "AdjustIfPossibleButAlwaysSpawn" "MultiplyWithRoot" null null))
        (else
          (bind _returnvalue_3 (`|SpawnActorFromClass` "/Game/MyContent/Player/BP_PlayerCharacter.BP_PlayerCharacter_C" _returnvalue "AdjustIfPossibleButAlwaysSpawn" "MultiplyWithRoot" null null)))))
    (`self.CreateWidgets`)
    (bind _asbp_game_instance (cast `/Game/MyContent/Core/BP_GameInstance` (`GameplayStatics.GetGameInstance`)))
    (`/Game/MyContent/Core/BP_GameInstance.TryLoadGame` _asbp_game_instance)
    (`self.OnInitalise`)))

(event `OnGameLoaded`
  (bind (_currentlevel_currentlevel _currentlevel_tag _currentlevel_levelstounstream) (break `/Game/MyContent/SaveGame/S_LevelData` (`/Game/MyContent/SaveGame/BP_SaveGame.CurrentLevel` (`/Game/MyContent/Core/BP_GameInstance.SavedGame` (`self.GameInstanceRef`)))))
  (`self.StreamLevel` _currentlevel_currentlevel _currentlevel_tag)
  (`self.UnstreamLevels` _currentlevel_levelstounstream))

(event `SpawnPlayers`
  (bind _worlddata_playerlocation (break `/Game/MyContent/SaveGame/S_WorldData` (`/Game/MyContent/SaveGame/BP_SaveGame.WorldData` (`/Game/MyContent/Core/BP_GameInstance.SavedGame` (`self.GameInstanceRef`)))))
  ; Spawn In Players
  (`self.CheckPlayerLocationValid`)
  (`GameplayStatics.CreatePlayer` 0)
  (set `self.PlayerIndex` 0)
  (bind _returnvalue (`|SpawnActorFromClass` "/Game/MyContent/Player/BP_PlayerCharacter.BP_PlayerCharacter_C" (`|GetArrayItem` _worlddata_playerlocation) "AlwaysSpawn" "MultiplyWithRoot" null null))
  (bind _asbp_player_controller (cast `/Game/MyContent/Player/BP_PlayerController` (`GameplayStatics.GetPlayerController` 0)))
  (set `/Game/MyContent/Player/BP_PlayerController.PlayerIndex` 0 _asbp_player_controller)
  (`Controller.Possess` _asbp_player_controller _returnvalue)
  ;[0.15 0 0 0.5] RUN  COMPLETED - PLAYER HAS SPAWNED
  (`self.Completed`))

(event `self.ReceiveBeginPlay`
  ;[0.15 0.002713 1.1e-05 0.5] Begin Play
  (`self.CreateRefsAndBinds`)
  (`self.CreateWidgets`)
  (`/Game/MyContent/Core/BP_GameInstance.TryLoadGame` (`self.GameInstanceRef`)))

(event `self.ReceiveTick`
  (params (DeltaSeconds :type "Float (single-precision)"))
  ; Ikd old nodes? not sure
)

(event `UnstreamLevels`
  (params (Levels :type "Array of Name"))
  (bind (_currentlevel_currentlevel _currentlevel_tag _currentlevel_levelstounstream) (break `/Game/MyContent/SaveGame/S_LevelData` (`/Game/MyContent/SaveGame/BP_SaveGame.CurrentLevel` (`/Game/MyContent/Core/BP_GameInstance.SavedGame` (`self.GameInstanceRef`)))))
  ;[0.15 0.0218 0.0132 0.5] Unstream Not Used Levels
  (`|ExecutionSequence`
    (:`then_0`
      (for _array_element _currentlevel_levelstounstream
        (`GameplayStatics.UnloadStreamLevel` _array_element)))
    (:`then_1`
      (bind _outactors (`GameplayStatics.GetAllActorsOfClass` "/Game/MyContent/Enemies/BP_Enemy.BP_Enemy_C"))
      (for _array_element_2 _outactors
        (`self.K2_DestroyActor` _array_element_2)))))

(event `Completed`
  (`/Game/MyContent/Core/BP_GameInstance.LoadPlayerData` (`self.GameInstanceRef`))
  (`UserWidget.AddToViewport` (`self.GM_HUD`) 1)
  (`self.OnInitalise`)
  ;[0.15 0.01048 0.01242 0.5] Initialise has to run somehwere here, preferably after most important stuff is called
  (`|ExecutionSequence`
    (:`then_0`
      (`KismetArrayLibrary.Array_Clear` (`self.EnemiesInLevel`))
      ;[0.15 0.1341 0.05233 0.5] Get All enemies and play sound cue
      (`KismetSystemLibrary.K2_SetTimerDelegate` (`|CreateDelegate` :!event `GetAllAliveEnemies`) 10.0 true))
    (:`then_1`
      ;[0.03646 0.03646 0.03646 0.5] Remove Loading Screen After Delay
      (`KismetSystemLibrary.Delay` 1.0)
      (`Widget.RemoveFromParent` (`self.GM_LoadingScreen`)))))

(event `StreamLevel`
  (params (`Level ` :type Name) (Tag :type Name))
  (bind (_currentlevel_currentlevel _currentlevel_tag _currentlevel_levelstounstream) (break `/Game/MyContent/SaveGame/S_LevelData` (`/Game/MyContent/SaveGame/BP_SaveGame.CurrentLevel` (`/Game/MyContent/Core/BP_GameInstance.SavedGame` (`self.GameInstanceRef`)))))
  ;[0.15 0.01472 0.01043 0.5] Stream In New level
  (`UserWidget.AddToViewport` (`self.GM_LoadingScreen`) 4)
  (`GameplayStatics.LoadStreamLevel` _currentlevel_currentlevel true true)
  (`self.SpawnPlayers`)
  (`self.OnLevelStreamed`))

(fn `CheckPlayerLocationValid`
  (bind _worlddata_playerlocation (break `/Game/MyContent/SaveGame/S_WorldData` (`/Game/MyContent/SaveGame/BP_SaveGame.WorldData` (`/Game/MyContent/Core/BP_GameInstance.SavedGame` (`self.GameInstanceRef`)))))
  (if (`KismetArrayLibrary.Array_IsEmpty` _worlddata_playerlocation)
    (`/Game/MyContent/Core/BP_GameInstance.GetPlayerStartLocations` (`self.GameInstanceRef`))
    (return)
    (else
      (return))))

(fn `CreateRefsAndBinds`
  (bind _asbp_game_instance (cast `/Game/MyContent/Core/BP_GameInstance` (`GameplayStatics.GetGameInstance`)))
  (bind _output_get (set `self.GameInstanceRef` _asbp_game_instance))
  (add `/Game/MyContent/Core/BP_GameInstance.OnGameLoaded` _output_get (`|CreateDelegate` :!event `OnGameLoaded`))
  (bind _returnvalue (`|CreateWidget` "/Game/MyContent/Menus/MainMenu/BP_UI_LoadingScreen.BP_UI_LoadingScreen_C"))
  (bind _output_get_2 (set `self.GM_LoadingScreen` _returnvalue))
  (`UserWidget.AddToViewport` _output_get_2 4)
  (add `self.OnLevelStreamed` (`|CreateDelegate` :!event `OnLevelStreamedGM`)))

(fn `CreateWidgets`
  ; Menu? idk what this does honestly
  (bind _returnvalue (`|CreateWidget` "/Game/MyContent/Player/HUD/BP_UI_HUD.BP_UI_HUD_C"))
  (set `self.GM_Menu` _returnvalue)
  (bind _returnvalue_2 (`|CreateWidget` "/Game/MyContent/Player/HUD/BP_UI_HUD.BP_UI_HUD_C"))
  (set `self.GM_HUD` _returnvalue_2)
  (bind _returnvalue_3 (`|CreateWidget` "/Game/MyContent/Menus/PauseMenu/BP_UI_PauseMenu.BP_UI_PauseMenu_C"))
  (set `self.GM_PauseMenu` _returnvalue_3)
  (bind _returnvalue_4 (`|CreateWidget` "/Game/MyContent/Menus/DeathMenu/BP_UI_DeathScreen.BP_UI_DeathScreen_C"))
  (set `self.GM_DeathScreen` _returnvalue_4)
  (bind _returnvalue_5 (`|CreateWidget` "/Game/MyContent/Menus/SettingsMenu/BP_UW_SettingsMenu.BP_UW_SettingsMenu_C"))
  (set `self.GM_SettingsMenu` _returnvalue_5))

(fn `GetAllAliveEnemies`
  (if (and (not (`KismetArrayLibrary.Array_IsEmpty` (`self.EnemiesInLevel`))) (>= (`KismetArrayLibrary.Array_Length` (`self.EnemiesInLevel`)) 2))
    (for _ (range 3)
      (`/Game/MyContent/Enemies/BP_Enemy.SetVoiceCueTimer` (`KismetArrayLibrary.Array_Random` (`self.EnemiesInLevel`))))))

(fn `OnLevelStreamedGM`)

(fn `PlayersDeadAddMenu`
  (bind _playersdead (`self.PlayersDead`))
  (`KismetArrayLibrary.Array_Clear` (`self.PlayersDead`))
  (bind _outactors (`GameplayStatics.GetAllActorsOfClass` "/Game/MyContent/Player/BP_PlayerCharacter.BP_PlayerCharacter_C"))
  (for _array_element _outactors
    (`KismetArrayLibrary.Array_Add` (`self.PlayersDead`) (not (`/Game/MyContent/Core/BP_AC_Stats.IsAlive` (`/Game/MyContent/Player/BP_PlayerCharacter.StatComponent` _array_element)))))
  (if (and (`|GetArrayItem` _playersdead) (`|GetArrayItem` _playersdead 1))
    (`UserWidget.AddToViewport` (`self.GM_DeathScreen`) 0)
    (for _array_element_2 _outactors
      (`/Game/MyContent/Player/BP_PlayerCharacter.RemoveInput` _array_element_2 false (`|MakeArray` "/Game/MyContent/Player/Input/IMC_Core.IMC_Core" :!type "InputMappingContext Object Reference")))))

(fn `SetPlayerLocations`
  (params (Tag :type Name))
  (bind _outactors (`GameplayStatics.GetAllActorsOfClassWithTag` "/Script/Engine.PlayerStart" Tag))
  (bind _outactors_2 (`GameplayStatics.GetAllActorsOfClass` "/Game/MyContent/Player/BP_PlayerCharacter.BP_PlayerCharacter_C"))
  (`self.K2_SetActorTransform` (`|GetArrayItem` _outactors_2) (`self.GetTransform` (`|GetArrayItem` _outactors)) false true)
  (`self.K2_SetActorTransform` (`|GetArrayItem` _outactors_2 1) (`self.GetTransform` (`|GetArrayItem` _outactors 1)) false true))

(fn `TogglePause`
  (if (not (`GameplayStatics.IsGamePaused`))
    (`UserWidget.AddToViewport` (`self.GM_PauseMenu`) 3)
    (`GameplayStatics.SetGamePaused` true)
    (else
      (`Widget.RemoveFromParent` (`self.GM_PauseMenu`))
      (`Widget.RemoveFromParent` (`self.GM_SettingsMenu`))
      (`GameplayStatics.SetGamePaused` false)
      (bind _asbp_player_controller (cast `/Game/MyContent/Player/BP_PlayerController` (`GameplayStatics.GetPlayerController` 0)))
      (`WidgetBlueprintLibrary.SetInputMode_GameOnly` _asbp_player_controller))))

(fn `ToggleSettings`
  (if (not (`Widget.IsInViewport` (`self.GM_SettingsMenu`)))
    (`UserWidget.AddToViewport` (`self.GM_SettingsMenu`) 5)
    (else
      (`Widget.RemoveFromParent` (`self.GM_SettingsMenu`)))))

(fn `UserConstructionScript`)