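; BP_GM_Menu, by its name the menu game mode, chooses between the launch intro and the main menu on BeginPlay.
; A first-opened flag on BP_GameInstance makes the BP_UI_Launch widget show only once, with the cursor hidden.
; Later loads call AddMenu, which calls CreatePlayer, shows BP_UI_MainMenu with the cursor, and sets UI-only input focused on the Play button.
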(event `self.ReceiveBeginPlay`
  (bind _returnvalue (`GameplayStatics.GetPlayerController` 0))
  ; Intro Seqeunce
  (bind _asbp_game_instance (cast `/Game/MyContent/Core/BP_GameInstance` (`GameplayStatics.GetGameInstance`)))
  (if (not (`/Game/MyContent/Core/BP_GameInstance.GameFirstOpened` _asbp_game_instance))
    (set `/Game/MyContent/Core/BP_GameInstance.GameFirstOpened` true _asbp_game_instance)
    (bind _returnvalue_2 (`|CreateWidget` "/Game/MyContent/Menus/BP_UI_Launch.BP_UI_Launch_C"))
    (`UserWidget.AddToViewport` _returnvalue_2 4)
    (if (`KismetSystemLibrary.IsValid` _returnvalue)
      (set `PlayerController.bShowMouseCursor` false _returnvalue))
    (else
      (`self.AddMenu`))))

(event `AddMenu`
  (bind _returnvalue (`GameplayStatics.GetPlayerController` 0))
  (`GameplayStatics.CreatePlayer` 0)
  (bind _returnvalue_2 (`|CreateWidget` "/Game/MyContent/Menus/MainMenu/BP_UI_MainMenu.BP_UI_MainMenu_C"))
  (`UserWidget.AddToViewport` _returnvalue_2 0)
  (bind _bp_btn_play (`/Game/MyContent/Menus/MainMenu/BP_UI_MainMenu.BP_Btn_Play` _returnvalue_2))
  (`Widget.SetKeyboardFocus` _bp_btn_play)
  (set `PlayerController.bShowMouseCursor` true _returnvalue)
  (`WidgetBlueprintLibrary.SetInputMode_UIOnlyEx` _returnvalue _bp_btn_play))

(fn `UserConstructionScript`)