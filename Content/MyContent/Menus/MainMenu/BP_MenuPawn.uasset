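; Main menu pawn that moves along a fixed straight path, apparently to animate the menu camera.
; On BeginPlay a timeline lerps the actor location between two hard-coded points along X.
; When it finishes, a Reverse event replays it from the start, so the motion loops by snapping back despite the event's name.
; On possession by BP_PlayerController, it hides the mouse cursor.
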(event `InitMovement`
  (bind (_direction _newtrack_0) (`Timeline|TL_CameraMovement` :!via `PlayFromStart` :!label _label)
    (:`Update`
      (`self.K2_SetActorLocation` (`KismetMathLibrary.VLerp` (-800.0 545.0 110.0) (-600.0 545.0 110.0) _newtrack_0)))
    (:`Finished`
      (`self.Reverse`))))

(event `self.ReceiveBeginPlay`
  (`self.InitMovement`))

(event `Reverse`
  (goto _label :!via `PlayFromStart`))

(event `self.ReceivePossessed`
  (params (NewController :type "Controller Object Reference"))
  (bind _asbp_player_controller (cast `/Game/MyContent/Player/BP_PlayerController` NewController))
  (set `PlayerController.bShowMouseCursor` false _asbp_player_controller))

(fn `UserConstructionScript`)