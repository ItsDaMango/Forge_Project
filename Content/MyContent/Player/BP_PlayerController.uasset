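; Player controller for a two-player game that links each player to their BP_PlayerCharacter and HUD health bar.
; InitPlayer creates a radial progress bar, colours it by PlayerIndex and adds it to that player's slot on the game mode's HUD.
; Possession registers the Enhanced Input mapping contexts and, after a short delay, passes PlayerIndex to the character.
; Input actions forward to the character or its camera's debug, and RespawnPlayer spawns and possesses a new character.
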(event `InitPlayer`
  (bind _gm_hud (`self.GM_HUD`))
  (bind _asbp_gm_main (cast `/Game/MyContent/Core/BP_GM_Main` (`GameplayStatics.GetGameMode`)))
  (set `self.GM_HUD` (`/Game/MyContent/Core/BP_GM_Main.GM_HUD` _asbp_gm_main))
  (if (<= (`self.PlayerIndex`) 1)
    ; p1
    (bind _returnvalue (`|CreateWidget` "/Game/MyContent/Player/HUD/BP_UW_RadProgBar.BP_UW_RadProgBar_C" self))
    (bind _output_get (set `self.PlayerHP` _returnvalue))
    (set `/Game/MyContent/Player/HUD/BP_UW_RadProgBar.BlockColour` (struct :`R` 1.0 :`B` 0.02046 :`A` 1.0) _output_get)
    (`PanelWidget.AddChild` (`/Game/MyContent/Player/HUD/BP_UI_HUD.SB_Player1` _gm_hud) _output_get)
    (else
      (bind _returnvalue_2 (`|CreateWidget` "/Game/MyContent/Player/HUD/BP_UW_RadProgBar.BP_UW_RadProgBar_C" self))
      (bind _output_get_2 (set `self.PlayerHP` _returnvalue_2))
      (set `/Game/MyContent/Player/HUD/BP_UW_RadProgBar.BlockColour` (struct :`G` 1.0 :`B` 0.123169 :`A` 1.0) _output_get_2)
      (`PanelWidget.AddChild` (`/Game/MyContent/Player/HUD/BP_UI_HUD.SB_Player2` _gm_hud) _output_get_2))))

(event `self.ReceivePossess`
  (params (PossessedPawn :type "Pawn Object Reference"))
  (bind _asbp_player_character (cast `/Game/MyContent/Player/BP_PlayerCharacter` PossessedPawn))
  (set `self.PlayerRef` _asbp_player_character)
  (`self.SetDefaults`)
  (`KismetSystemLibrary.K2_SetTimerDelegate` (`|CreateDelegate` :!event `InitPlayer`) 0.1)
  (`KismetSystemLibrary.Delay` 0.1)
  (set `/Game/MyContent/Player/BP_PlayerCharacter.PlayerIndex` (`self.PlayerIndex`) (`self.PlayerRef`)))

(event `EnhancedInput|/Game/MyContent/Player/Input/IA_Move`
  (params (ActionValue :type "Vector2D Structure") (ElapsedSeconds :type "Float (double-precision)") (TriggeredSeconds :type "Float (double-precision)") (InputAction :type "InputAction Object Reference" :default "/Game/MyContent/Player/Input/IA_Move.IA_Move"))
  (:`Triggered`
    (`/Game/MyContent/Player/BP_PlayerCharacter.MovePlayer` (`self.PlayerRef`) ActionValue :!label _label))
  (:`Ongoing`
    (goto _label))
  (:`Canceled`
    (goto _label)))

(event `EnhancedInput|/Game/MyContent/Player/Input/IA_Rotate`
  (params (ActionValue :type "Vector2D Structure") (ElapsedSeconds :type "Float (double-precision)") (TriggeredSeconds :type "Float (double-precision)") (InputAction :type "InputAction Object Reference" :default "/Game/MyContent/Player/Input/IA_Rotate.IA_Rotate"))
  (:`Triggered`
    (`/Game/MyContent/Player/BP_PlayerCharacter.RotatePlayer` (`self.PlayerRef`) ActionValue)))

(event `EnhancedInput|/Game/MyContent/Player/Input/IA_Dash`
  (params (ActionValue :type Boolean) (ElapsedSeconds :type "Float (double-precision)") (TriggeredSeconds :type "Float (double-precision)") (InputAction :type "InputAction Object Reference" :default "/Game/MyContent/Player/Input/IA_Dash.IA_Dash"))
  (:`Triggered`
    (`/Game/MyContent/Player/BP_PlayerCharacter.Dash` (`self.PlayerRef`))))

(event `EnhancedInput|/Game/MyContent/Player/Input/IA_Debug`
  (params (ActionValue :type Boolean) (ElapsedSeconds :type "Float (double-precision)") (TriggeredSeconds :type "Float (double-precision)") (InputAction :type "InputAction Object Reference" :default "/Game/MyContent/Player/Input/IA_Debug.IA_Debug"))
  (:`Triggered`
    (`/Game/MyContent/Player/BP_CameraManager.DebugOn` (`/Game/MyContent/Player/BP_PlayerCharacter.CameraRef` (`self.PlayerRef`)))))

(event `EnhancedInput|/Game/MyContent/Player/Input/IA_PrimaryAttack`
  (params (ActionValue :type Boolean) (ElapsedSeconds :type "Float (double-precision)") (TriggeredSeconds :type "Float (double-precision)") (InputAction :type "InputAction Object Reference" :default "/Game/MyContent/Player/Input/IA_PrimaryAttack.IA_PrimaryAttack"))
  (:`Triggered`
    (`/Game/MyContent/Player/BP_PlayerCharacter.PrimaryAttack` (`self.PlayerRef`))))

(fn `AddInput`
  (params (MappingContext :type "InputMappingContext Object Reference") (`Options Ignore All Pressed Keys Until Release` :type Boolean) (Priority :type Integer))
  (`EnhancedInputSubsystemInterface.AddMappingContext` (subsystem `EnhancedInputLocalPlayerSubsystem`) MappingContext Priority (make `ModifyContextOptions` `Options Ignore All Pressed Keys Until Release`)))

(fn `RemoveInputs`
  (params (`Options Ignore All Pressed Keys Until Release` :type Boolean) (MappingContext :type "InputMappingContext Object Reference"))
  (`EnhancedInputSubsystemInterface.RemoveMappingContext` (subsystem `EnhancedInputLocalPlayerSubsystem`) MappingContext (make `ModifyContextOptions` `Options Ignore All Pressed Keys Until Release`)))

(fn `RespawnPlayer`
  (params (SpawnTransform :type "Transform Structure"))
  (bind _returnvalue (`|SpawnActorFromClass` "/Game/MyContent/Player/BP_PlayerCharacter.BP_PlayerCharacter_C" SpawnTransform "Undefined" "MultiplyWithRoot" null null))
  (`self.Possess` _returnvalue))

(fn `SetDefaults`
  (set `/Game/MyContent/Player/BP_PlayerCharacter.PlayerController` self (`self.PlayerRef`))
  (for _array_element (`|MakeArray` "/Game/MyContent/Player/Input/IMC_Movement.IMC_Movement" "/Game/MyContent/Player/Input/IMC_Menu.IMC_Menu" "/Game/MyContent/Player/Input/IMC_Core.IMC_Core" "/Game/MyContent/Player/Input/IMC_Combat.IMC_Combat" :!type "InputMappingContext Object Reference")
    (`self.AddInput` _array_element)))

(fn `SetUniques`
  (params (PlayerHUD :type "/Game/MyContent/Player/HUD/BP_UW_RadProgBar Object Reference") (GameMode :type "/Game/MyContent/Core/BP_GM_Main Object Reference"))
  (set `self.PlayerHP` PlayerHUD)
  (set `self.GameMode` GameMode))

(fn `UserConstructionScript`)