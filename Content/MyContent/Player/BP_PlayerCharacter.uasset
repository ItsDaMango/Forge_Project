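; Player character for two-player melee combat, with camera-relative movement, dash, death and respawn at half health.
; Dash moves the capsule on a timeline, ignoring some collision channels when a sphere trace ahead is clear, while a line trace gates dashing against the camera manager.
; Montages and timers pace attacks through a child-actor weapon; StatComponent handles health, driving HUD hit flashes or death.
; Tick saves grounded locations to recover from falls.
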(event `self.ReceiveTick`
  (params (DeltaSeconds :type "Float (single-precision)"))
  (bind _charactermovement (`self.CharacterMovement`))
  (`|ExecutionSequence`
    (:`then_0`
      ; Set Actor Last location if they were on the ground and NOT falling
      (`KismetSystemLibrary.Delay` 2.0)
      (if (and (`NavMovementComponent.IsMovingOnGround` _charactermovement) (not (`NavMovementInterface.IsFalling` _charactermovement)))
        (set `self.LastLoc` (`self.K2_GetActorLocation`))))
    (:`then_1`
      ; if actor IS falling for more than X seconds (delay) set their location back to the last loc
      (if (`NavMovementInterface.IsFalling` (`self.CharacterMovement`))
        (`KismetSystemLibrary.Delay` 3.0)
        (`self.K2_SetActorLocation` (`self.LastLoc`) false true)))))

(event `DebugOn`
  ;[0.7135 0.2454 0 0.5] Debug Mode On/Off
  (`/Engine/EditorBlueprintResources/StandardMacros.FlipFlop`
    (:`A`
      (`self.DebugMode` true))
    (:`B`
      (`self.DebugMode` false))))

(event `PlayDash`
  (bind (_direction _alpha) (`Timeline|TL_Dash` :!via `PlayFromStart`)
    (:`Update`
      (`self.K2_SetActorLocation` (`KismetMathLibrary.VLerp` (`self.K2_GetActorLocation`) (+ (`self.K2_GetActorLocation`) (* (`self.GetActorForwardVector`) 25.0)) _alpha) true))))

(event `self.ReceiveBeginPlay`
  ;[0 0.8902 1 0.5] Event Begin Play
  (bind _asbp_weapon (cast `/Game/MyContent/Weapons/BP_Weapon` (`ChildActorComponent.ChildActor` (`self.WeaponActorComponent`))))
  (set `/Game/MyContent/Weapons/BP_Weapon.ClassToIgnore` (`|MakeArray` "BP_PlayerCharacter_C" :!type "Actor Class Reference") _asbp_weapon)
  (bind _returnvalue (`|CreateWidget` "/Game/MyContent/Player/HUD/BP_UW_SSText.BP_UW_SSText_C"))
  (bind _output_get (set `self.PlayerRespawnWidget` _returnvalue))
  (`WidgetComponent.SetWidget` (`self.Widget`) _output_get))

(event `self.ReceivePossessed`
  (params (NewController :type "Controller Object Reference")))

(event `self.ReceiveAnyDamage`
  (params (Damage :type "Float (single-precision)") (DamageType :type "DamageType Object Reference") (InstigatedBy :type "Controller Object Reference") (DamageCauser :type "Actor Object Reference"))
  ;[1 0 0 0.5] On Damage
  (`/Game/MyContent/Core/BP_AC_Stats.DamageHealth` (`self.StatComponent`) Damage)
  (set `self.bCanBeDamaged` false)
  (if (not (`/Game/MyContent/Core/BP_AC_Stats.IsAlive` (`self.StatComponent`)))
    (`self.Death` DamageCauser)
    (`KismetSystemLibrary.Delay` 2.0)
    (`SceneComponent.SetVisibility` (`self.Widget`) true false)
    (else
      (`self.PlayHitReact`))))

(event `self.Box.OnComponentBeginOverlap`
  (params (OverlappedComponent :type "PrimitiveComponent Object Reference") (OtherActor :type "Actor Object Reference") (OtherComp :type "PrimitiveComponent Object Reference") (OtherBodyIndex :type Integer) (bFromSweep :type Boolean) (SweepResult :type "HitResult Structure (by ref)")))

(event `self.Box.OnComponentEndOverlap`
  (params (OverlappedComponent :type "PrimitiveComponent Object Reference") (OtherActor :type "Actor Object Reference") (OtherComp :type "PrimitiveComponent Object Reference") (OtherBodyIndex :type Integer)))

(fn `ActivateWeaponDamage`
  (bind _asbp_weapon (cast `/Game/MyContent/Weapons/BP_Weapon` (`ChildActorComponent.ChildActor` (`self.WeaponActorComponent`))))
  (`/Game/MyContent/Weapons/BP_Weapon.ActivateDamage` _asbp_weapon))

(fn `AddInput`
  (params (MappingContext :type "InputMappingContext Object Reference") (`Options Ignore All Pressed Keys Until Release` :type Boolean) (Priority :type Integer))
  (`/Game/MyContent/Player/BP_PlayerController.AddInput` (`self.PlayerController`) MappingContext `Options Ignore All Pressed Keys Until Release` Priority))

(fn `CheckCollision`
  (bind (_strace_tracecomplex _strace_tracetype _strace_tracemode) (break `/Game/MyContent/Player/S_Trace` (`self.STrace`)))
  (bind _bdebugon (`self.bDebugOn`))
  (bind _outhit (`KismetSystemLibrary.LineTraceSingle` (+ (+ (`self.K2_GetActorLocation`) (* (`KismetMathLibrary.GetForwardVector` (`self.K2_GetActorRotation`)) 1.0)) (0.0 0.0 80.0)) (+ (+ (`self.K2_GetActorLocation`) (* (`KismetMathLibrary.GetForwardVector` (`self.K2_GetActorRotation`)) 500.0)) (0.0 0.0 80.0)) _strace_tracetype _strace_tracecomplex (`|MakeArray` self :!type "Actor Object Reference") _strace_tracemode))
  (cast `/Game/MyContent/Player/BP_CameraManager` (`.HitActor` (`GameplayStatics.BreakHitResult` _outhit))
    (:`then`
      (set `self.CanDash` false)
      (if _bdebugon
        (`KismetSystemLibrary.PrintString` "C - Not")))
    (:`CastFailed`
      (set `self.CanDash` true)
      (if _bdebugon
        (`KismetSystemLibrary.PrintString` "C - Can")))))

(fn `CheckIfDashObstructed`
  (bind (_strace_tracecomplex _strace_tracetype _strace_tracemode) (break `/Game/MyContent/Player/S_Trace` (`self.STrace`)))
  (bind (_outhit _returnvalue) (`KismetSystemLibrary.SphereTraceSingle` (+ (`self.K2_GetActorLocation`) (* (`KismetMathLibrary.GetForwardVector` (`self.K2_GetActorRotation`)) 450.0)) (+ (`self.K2_GetActorLocation`) (* (`KismetMathLibrary.GetForwardVector` (`self.K2_GetActorRotation`)) 510.0)) 50.0 _strace_tracetype _strace_tracecomplex (`|MakeArray` self :!type "Actor Object Reference") _strace_tracemode))
  (if (not _returnvalue)
    (`self.SetCollisionResponse` "ECR_Ignore" (`|MakeArray` "ECC_WorldDynamic" "ECC_Pawn" "ECC_GameTraceChannel2" :!type "ECollisionChannel Enum") (`self.CapsuleComponent`)))
  (return))

(fn `Dash`
  (`self.CheckIfDashObstructed`)
  (if (and (not (`self.IsDashing`)) (`self.CanDash`))
    (if (`NavMovementComponent.IsMovingOnGround` (`self.CharacterMovement`))
      (set `self.CanDash` false)
      (set `self.IsDashing` true)
      (`AnimInstance.Montage_Play` (`SkeletalMeshComponent.GetAnimInstance` (`self.Mesh`)) "/Game/MyContent/Player/Characters/Animations/Male_Dash_Montage.Male_Dash_Montage" 1.2 "Duration" 0.0 false)
      (`KismetSystemLibrary.K2_SetTimerDelegate` (`|CreateDelegate` :!event `ResetDash`) 0.25)
      (`self.PlayDash`))))

(fn `DeactivateWeaponDamage`
  (bind _asbp_weapon (cast `/Game/MyContent/Weapons/BP_Weapon` (`ChildActorComponent.ChildActor` (`self.WeaponActorComponent`))))
  (`/Game/MyContent/Weapons/BP_Weapon.DeactivateDamage` _asbp_weapon))

(fn `Death`
  (params (DamageCauser :type "Actor Object Reference"))
  (bind _array (`|MakeArray` "ECC_Visibility" "ECC_Pawn" :!type "ECollisionChannel Enum"))
  (set `self.CanRespawn` true)
  (set `self.CanAttack` false)
  (`self.RemoveInput` false (`|MakeArray` "/Game/MyContent/Player/Input/IMC_Combat.IMC_Combat" "/Game/MyContent/Player/Input/IMC_Movement.IMC_Movement" :!type "InputMappingContext Object Reference"))
  (`self.SetCollisionResponse` "ECR_Ignore" _array (`self.Mesh`))
  (`self.SetCollisionResponse` "ECR_Ignore" _array (`self.CapsuleComponent`)))

(fn `DebugMode`
  (params (Condition :type Boolean))
  (if Condition
    (`SceneComponent.SetHiddenInGame` (`self.CapsuleComponent`) false false)
    (`SceneComponent.SetHiddenInGame` (`self.Box`) false false)
    (set `self.bDebugOn` true)
    (set `self.STrace` (make `/Game/MyContent/Player/S_Trace` false "TraceTypeQuery1" "ForDuration"))
    (else
      (`SceneComponent.SetHiddenInGame` (`self.CapsuleComponent`) true false)
      (`SceneComponent.SetHiddenInGame` (`self.Box`) true false)
      (set `self.bDebugOn` false)
      (set `self.STrace` (make `/Game/MyContent/Player/S_Trace` false)))))

(fn `DisableAttack`
  (params (Duration :type "Float (double-precision)"))
  (set `self.CanAttack` false)
  (`self.RemoveInput` false (`|MakeArray` "/Game/MyContent/Player/Input/IMC_Combat.IMC_Combat" :!type "InputMappingContext Object Reference"))
  (bind _returnvalue (`KismetSystemLibrary.K2_SetTimerDelegate` (`|CreateDelegate` :!event `EnableAttack`) Duration))
  (set `self.THEnableAttack` _returnvalue))

(fn `EnableAttack`
  (set `self.CanAttack` true)
  (set `self.bCanBeDamaged` true)
  (`self.AddInput` "/Game/MyContent/Player/Input/IMC_Combat.IMC_Combat")
  (`KismetSystemLibrary.K2_ClearAndInvalidateTimerHandle` (`self.THEnableAttack`)))

(fn `InitialiseWeapon`
  (bind _asbp_weapon (cast `/Game/MyContent/Weapons/BP_Weapon` (`ChildActorComponent.ChildActor` (`self.WeaponActorComponent`))))
  (`self.SetOwner` _asbp_weapon self)
  (set `/Game/MyContent/Weapons/BP_Weapon.Damage` 10.0 _asbp_weapon))

(fn `MovePlayer`
  (params (Axis :type "Vector2D Structure"))
  (bind (_playeraxis_x _playeraxis_y) (`KismetMathLibrary.BreakVector2D` (`self.PlayerAxis`)))
  (bind (_returnvalue_roll _returnvalue_pitch _returnvalue_yaw) (`KismetMathLibrary.BreakRotator` (`self.K2_GetActorRotation` (`self.CameraRef`))))
  (bind _returnvalue (`KismetMathLibrary.MakeRotator` 0.0 0.0 _returnvalue_yaw))
  (if (not (`self.IsDashing`))
    (set `self.PlayerAxis` Axis)
    (`|ExecutionSequence`
      (:`then_0`
        (`self.AddMovementInput` (`KismetMathLibrary.GetRightVector` _returnvalue) _playeraxis_x))
      (:`then_1`
        (`self.AddMovementInput` (`KismetMathLibrary.GetForwardVector` _returnvalue) _playeraxis_y)))))

(fn `PlayHitReact`
  (bind _gm_hud (`/Game/MyContent/Player/BP_PlayerController.GM_HUD` (`self.PlayerController`)))
  (if (<= (`self.PlayerIndex`) 1)
    (`UserWidget.PlayAnimation` _gm_hud (`/Game/MyContent/Player/HUD/BP_UI_HUD.P1_Hitflash` _gm_hud) 0.0 1 "Forward" 1.0 false)
    (else
      (`UserWidget.PlayAnimation` _gm_hud (`/Game/MyContent/Player/HUD/BP_UI_HUD.P2_Hitflash` _gm_hud) 0.0 1 "Forward" 1.0 false))))

(fn `PlayMontage`
  (returns (Duration :type "Float (single-precision)"))
  (bind _returnvalue (`AnimInstance.Montage_Play` (`SkeletalMeshComponent.GetAnimInstance` (`self.Mesh`)) "/Game/MyContent/Player/Characters/Animations/Male_Attack_Upper_Montage.Male_Attack_Upper_Montage" 1.0 "Duration" 0.0 true))
  (return (/ _returnvalue 2.0)))

(fn `PrimaryAttack`
  (if (`self.CanAttack`)
    (set `self.CanAttack` false)
    (bind _duration (`self.PlayMontage`))
    (`KismetSystemLibrary.K2_SetTimerDelegate` (`|CreateDelegate` :!event `ResetAttack`) _duration)))

(fn `RemoveInput`
  (params (`Options Ignore All Pressed Keys Until Release` :type Boolean) (Array :type "Array of InputMappingContext Object Reference"))
  (for _array_element Array
    (`/Game/MyContent/Player/BP_PlayerController.RemoveInputs` (`self.PlayerController`) `Options Ignore All Pressed Keys Until Release` _array_element)))

(fn `ResetAttack`
  (set `self.CanAttack` true))

(fn `ResetDash`
  (set `self.IsDashing` false)
  (`self.SetCollisionResponse` "ECR_Block" (`|MakeArray` "ECC_WorldDynamic" "ECC_Pawn" "ECC_GameTraceChannel2" :!type "ECollisionChannel Enum") (`self.CapsuleComponent`))
  (set `self.CanDash` true))

(fn `Respawn`
  (locals (LMontageLength :type "Float (single-precision)" :default 2.97) (LPlayRate :type "Float (single-precision)" :default 2.0))
  (bind _statcomponent (`self.StatComponent`))
  (if (and (not (`/Game/MyContent/Core/BP_AC_Stats.IsAlive` (`self.StatComponent`))) (`self.CanRespawn`))
    (set `self.CanRespawn` false)
    (bind _returnvalue (`AnimInstance.Montage_Play` (`SkeletalMeshComponent.GetAnimInstance` (`self.Mesh`)) "/Game/Sword_Animations/Animations/Sequence2/08_Hit/02_Hit_Combat/Hit_Combat_Death_Seq_Montage1.Hit_Combat_Death_Seq_Montage1" (`local.LPlayRate`) "MontageLength" (`local.LMontageLength`) true))
    (`KismetSystemLibrary.K2_SetTimerDelegate` (`|CreateDelegate` :!event `SetCanBeDamaged`) (/ _returnvalue (`local.LPlayRate`)))
    (`/Game/MyContent/Core/BP_AC_Stats.SetHealth` _statcomponent (/ (`/Game/MyContent/Core/BP_AC_Stats.MaxHealth` _statcomponent) 2.0))
    (`SceneComponent.SetVisibility` (`self.Widget`) false false)))

(fn `RotatePlayer`
  (params (Axis :type "Vector2D Structure")))

(fn `SetCanBeDamaged`
  (set `self.bCanBeDamaged` true)
  (set `self.CanAttack` true)
  (`self.AddInput` "/Game/MyContent/Player/Input/IMC_Combat.IMC_Combat")
  (`self.AddInput` "/Game/MyContent/Player/Input/IMC_Movement.IMC_Movement")
  (`KismetSystemLibrary.PrintString` "Inputs back"))

(fn `SetCollisionCheck`
  (`KismetSystemLibrary.K2_SetTimerDelegate` (`|CreateDelegate` :!event `CheckCollision`) 0.1 true true))

(fn `SetCollisionResponse`
  (params (NewResponse :type "ECollisionResponse Enum" :default "ECR_Ignore") (Array :type "Array of ECollisionChannel Enum") (Component :type "PrimitiveComponent Object Reference"))
  (for _array_element Array
    (`PrimitiveComponent.SetCollisionResponseToChannel` Component _array_element NewResponse)))

(fn `UserConstructionScript`)