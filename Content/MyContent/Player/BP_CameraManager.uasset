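; Shared two-player camera manager actor that becomes the view target and follows the players' midpoint.
; Looping timers and timelines drive it, lerping position and scaling spring-arm length with player separation within min/max limits.
; Sphere traces toward each player detect BP_Collision obstructions and swap their materials.
; Combat mode tilts the arm down, and a debug toggle shows traces and boxes; default-mode, alive and stationary checks are stubbed or unwired.
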(event `DebugOn`
  ;[1 0.9624 0 0.5] Debug Mode - Development Only
  (`/Engine/EditorBlueprintResources/StandardMacros.FlipFlop`
    (:`A`
      (`self.DebugMode` true))
    (:`B`
      (`self.DebugMode` false)
      (`KismetSystemLibrary.FlushPersistentDebugLines`)
      (`KismetSystemLibrary.FlushDebugStrings`))))

(event `self.ReceiveBeginPlay`
  ;[1 0.02604 0.02604 0.5] BeginPlay
  (bind _asbp_gm_main (cast `/Game/MyContent/Core/BP_GM_Main` (`GameplayStatics.GetGameMode`)))
  (add `/Game/MyContent/Core/BP_GM_Main.Initialise` _asbp_gm_main (`|CreateDelegate` :!event `InitCamera`)))

(event `InitCamera`
  ;[0.9427 0.9427 0.9427 0.5] Initilise Camera and call tick
  (`PlayerController.SetViewTargetWithBlend` (`GameplayStatics.GetPlayerController` 0) self 0.0 "VTBlend_Cubic" 0.0 false)
  (bind _outactors (`GameplayStatics.GetAllActorsOfClass` "/Game/MyContent/Player/BP_PlayerCharacter.BP_PlayerCharacter_C"))
  (set `self.PlayerRefs` _outactors)
  (`KismetSystemLibrary.K2_SetTimerDelegate` (`|CreateDelegate` :!event `GetActorCenterLocation`) 0.08 true)
  (bind _returnvalue (`KismetSystemLibrary.K2_SetTimerDelegate` (`|CreateDelegate` :!event `LerpToPlayers`) 0.01 true))
  (set `self.TH_LerpToPlayers` _returnvalue)
  (`KismetSystemLibrary.PrintString` "Hello"))

(event `SetObstructTimer`
  (`KismetSystemLibrary.K2_SetTimerDelegate` (`|CreateDelegate` :!event `CheckPlayerObstructed`) 0.15 true))

(event `LerpOutOfBounds`
  (bind _playerrefs (`self.PlayerRefs`))
  ; Lerp to Location over X time, for when players are too far but can still walk through map
  (bind (_direction _alpha) (`Timeline|TL_Bounds`)
    (:`Update`
      (`self.K2_SetActorLocation` (`KismetMathLibrary.VLerp` (`self.K2_GetActorLocation`) (/ (+ (`self.K2_GetActorLocation` (`|GetArrayItem` _playerrefs)) (`self.K2_GetActorLocation` (`|GetArrayItem` _playerrefs 1))) 2.0) _alpha)))))

(event `CombatMode`
  (bind (_direction _alpha) (`Timeline|Timeline`)
    (:`Update`
      (`SceneComponent.K2_SetWorldRotation` (`self.SpringArm`) (`KismetMathLibrary.RLerp` (struct :`Pitch` -20.0) (struct :`Pitch` -70.0) _alpha) false false)
      (set `self.MaxTargetLength` 2500.0)
      (set `self.MinTargetLength` 2000.0))))

(event `DefaultMode`)

(event `LerpToPlayers`
  (bind _returnvalue (`self.K2_GetActorLocation`))
  (bind (_playerscenterloc_x _playerscenterloc_y _playerscenterloc_z) (`KismetMathLibrary.BreakVector` (`self.PlayersCenterLoc`)))
  (bind (_direction _alpha) (`Timeline|Timeline_0` :!via `PlayFromStart`)
    (:`Update`
      (`self.K2_SetActorLocation` (`KismetMathLibrary.VLerp` _returnvalue (`KismetMathLibrary.MakeVector` _playerscenterloc_x _playerscenterloc_y (.z _returnvalue)) _alpha))
      (set `SpringArmComponent.TargetArmLength` (`KismetMathLibrary.Lerp` (`SpringArmComponent.TargetArmLength` (`self.SpringArm`)) (`self.PlayerTargetArm`) _alpha) (`self.SpringArm`)))))

(fn `CheckPlayerAlive`)

(fn `CheckPlayerObstructed`
  (bind (_tracecomplex _tracetype _tracemode) (break `/Game/MyContent/Player/S_Trace` (`self.TraceStruct`)))
  (for (_array_element _array_index) (`self.PlayerRefs`)
    (bind (_outhit _returnvalue) (`KismetSystemLibrary.SphereTraceSingle` (+ (`SceneComponent.K2_GetComponentLocation` (`self.Camera`)) (select `int` _array_index :`0` (0.0 200.0 0.0) :`1` (0.0 -200.0 0.0) :!type "Vector Structure")) (+ (- (`self.K2_GetActorLocation` _array_element) (50.0 15.0 0.0)) (0.0 0.0 100.0)) 60.0 _tracetype _tracecomplex (`self.ArrayIgnore`) _tracemode))
    (if _returnvalue
      (bind _asbp_collision (cast `/Game/MyContent/Interactibles/BP_Collision` (`.HitActor` (`GameplayStatics.BreakHitResult` _outhit)))
        (:`then`
          (set `self.HitObstruction` true)
          (`/Game/MyContent/Interactibles/BP_Collision.SetMaterial` _asbp_collision 1)
          (`/Game/MyContent/Interactibles/BP_Collision.ResetMaterial` _asbp_collision))
        (:`CastFailed`
          (set `self.HitObstruction` false)))
      (else
        (set `self.HitObstruction` false)))))

(fn `CheckPlayerStationary`)

(fn `DebugMode`
  (params (Condition :type Boolean))
  (if Condition
    (`SceneComponent.SetHiddenInGame` (`self.Box1`) false false)
    (`SceneComponent.SetHiddenInGame` (`self.Box`) false false)
    (`SceneComponent.SetHiddenInGame` (`self.ClipCollision`) false false)
    (`SceneComponent.SetHiddenInGame` (`self.Box2`) false false)
    (`SceneComponent.SetHiddenInGame` (`self.Box3`) false false)
    (set `self.TraceStruct` (make `/Game/MyContent/Player/S_Trace` false "TraceTypeQuery1" "ForDuration"))
    (else
      (`SceneComponent.SetHiddenInGame` (`self.ClipCollision`) true false)
      (`SceneComponent.SetHiddenInGame` (`self.Box`) true false)
      (`SceneComponent.SetHiddenInGame` (`self.Box1`) true false)
      (`SceneComponent.SetHiddenInGame` (`self.Box2`) true false)
      (`SceneComponent.SetHiddenInGame` (`self.Box3`) true false)
      (set `self.TraceStruct` (make `/Game/MyContent/Player/S_Trace` false)))))

(fn `GetActorCenterLocation`
  (bind _playerrefs (`self.PlayerRefs`))
  (bind _output (`|GetArrayItem` _playerrefs))
  (bind _output_2 (`|GetArrayItem` _playerrefs 1))
  (if (`self.bLerpTargetArm`)
    (set `self.PlayerTargetArm` (`KismetMathLibrary.FClamp` (* (`self.GetDistanceTo` _output _output_2) 2.0) (`self.MinTargetLength`) (`self.MaxTargetLength`)))
    (set `self.PlayersCenterLoc` (/ (+ (`self.K2_GetActorLocation` _output) (`self.K2_GetActorLocation` _output_2)) 2.0))))

(fn `UserConstructionScript`)