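; Second boss enemy Character with a child-actor weapon, montage-driven two-part attacks, and a timeline-offset jump with landing VFX.
; On possession it initialises level-scaled health, the health widget and weapon damage, and setting a target alerts its assigned camp.
; Damage feeds the stat component, flashing dynamic mesh materials through a timeline or triggering death.
; Death disables damage and spawns a portal to the next office level that unloads the boss level.
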(event `self.ReceivePossessed`
  (params (NewController :type "Controller Object Reference"))
  (`KismetSystemLibrary.Delay` 0.1)
  (`self.InitialiseStats`)
  (bind _asbp_weapon (cast `/Game/MyContent/Weapons/BP_Weapon` (`ChildActorComponent.ChildActor` (`self.WeaponActorComponent`))))
  (set `/Game/MyContent/Weapons/BP_Weapon.ClassToIgnore` (`self.Classes to IgnoreDamge`) _asbp_weapon)
  (set `/Game/MyContent/Weapons/BP_Weapon.Damage` 15.0 _asbp_weapon))

(event `self.ReceiveTick`
  (params (DeltaSeconds :type "Float (single-precision)")))

(event `PlayHitFlash`
  (bind (_direction _alpha) (`Timeline|TL_HitFlash` :!via `PlayFromStart`)
    (:`Update`
      (for _array_element (`self.MeshMaterials`)
        (`MaterialInstanceDynamic.SetScalarParameterValue` _array_element "HitFlashAlpha" _alpha)))))

(event `self.ReceiveBeginPlay`
  (`KismetSystemLibrary.K2_SetTimerDelegate` (`|CreateDelegate` :!event `HandleFaceTarget`) 0.001 true))

(event `self.ReceiveAnyDamage`
  (params (Damage :type "Float (single-precision)") (DamageType :type "DamageType Object Reference") (InstigatedBy :type "Controller Object Reference") (DamageCauser :type "Actor Object Reference"))
  (`self.OnTakeDamage` DamageCauser Damage))

(event `BossJmpOffset`
  (bind _returnvalue (`self.K2_GetActorLocation`))
  (`KismetSystemLibrary.Delay` 1.0)
  (bind (_direction _newtrack_0) (`Timeline|TL_JumpMoveOffset`)
    (:`Update`
      (`self.K2_SetActorRelativeLocation` (`KismetMathLibrary.VLerp` _returnvalue (+ _returnvalue (-40.0 0.0 0.0)) _newtrack_0)))))

(fn `ActivateDamage`
  (bind _asbp_weapon (cast `/Game/MyContent/Weapons/BP_Weapon` (`ChildActorComponent.ChildActor` (`self.WeaponActorComponent`))))
  (`/Game/MyContent/Weapons/BP_Weapon.ActivateDamage` _asbp_weapon))

(fn `ActivateWeaponVFX`
  (bind _weaponparticle (`self.WeaponParticle`))
  (`FXSystemComponent.SetColorParameter` _weaponparticle "P_Colour" (struct :`R` 100.0 :`G` 7.320368 :`A` 1.0))
  (`NiagaraComponent.SetVariableVec3` _weaponparticle "P_Vector" (* (`self.GetActorForwardVector`) 500.0))
  (`ActorComponent.Activate` (`self.WeaponParticle`) true))

(fn `Attack`
  (returns (ReturnValue :type "Float (single-precision)"))
  (set `self.Attacking` true)
  (if (`KismetArrayLibrary.Array_IsNotEmpty` (`self.AttackAnims`))
    (bind _returnvalue (`AnimInstance.Montage_Play` (`SkeletalMeshComponent.GetAnimInstance` (`self.Mesh`)) "/Game/MyContent/Boss_2/Anims/Boss2Attack1_Anim_Montage.Boss2Attack1_Anim_Montage" (`self.AttackSpeed`) "Duration" 0.0 false))
    (`KismetSystemLibrary.K2_SetTimerDelegate` (`|CreateDelegate` :!event `ResetAttacking`) _returnvalue)
    (return _returnvalue)))

(fn `Attack_Pt2`
  (returns (ReturnValue :type "Float (single-precision)"))
  (set `self.Attacking` true)
  (if (`KismetArrayLibrary.Array_IsNotEmpty` (`self.AttackAnims`))
    (bind _returnvalue (`AnimInstance.Montage_Play` (`SkeletalMeshComponent.GetAnimInstance` (`self.Mesh`)) "/Game/MyContent/Boss/Animations/Boss_Attack_SecondHit_Montage.Boss_Attack_SecondHit_Montage" (`self.AttackSpeed`) "Duration" 0.0 true))
    (`KismetSystemLibrary.K2_SetTimerDelegate` (`|CreateDelegate` :!event `ResetAttacking`) _returnvalue)
    (return _returnvalue)))

(fn `BossJump`
  (`self.BossJmpOffset`)
  (bind _returnvalue (`self.PlayAnimMontage` "/Game/MyContent/Boss/Animations/Boss_Jump_Montage.Boss_Jump_Montage" 0.9))
  (`KismetSystemLibrary.K2_SetTimerDelegate` (`|CreateDelegate` :!event `SpawnVFX`) (- _returnvalue 0.2)))

(fn `CreateDynamicMaterialInstance`
  (`KismetArrayLibrary.Array_Clear` (`self.MeshMaterials`))
  (for (_array_element _array_index) (`MeshComponent.GetMaterials` (`self.Mesh`))
    (bind _returnvalue (`PrimitiveComponent.CreateDynamicMaterialInstance` (`self.Mesh`) _array_index _array_element "None"))
    (`KismetArrayLibrary.Array_Add` (`self.MeshMaterials`) _returnvalue)))

(fn `DeactivateDamage`
  (bind _asbp_weapon (cast `/Game/MyContent/Weapons/BP_Weapon` (`ChildActorComponent.ChildActor` (`self.WeaponActorComponent`))))
  (`/Game/MyContent/Weapons/BP_Weapon.DeactivateDamage` _asbp_weapon))

(fn `Death`
  (set `self.bCanBeDamaged` false)
  (`PrimitiveComponent.SetCollisionResponseToChannel` (`self.CapsuleComponent`) "ECC_Pawn" "ECR_Ignore")
  (`PrimitiveComponent.SetCollisionEnabled` (`self.Mesh`) "PhysicsOnly")
  (`SceneComponent.SetVisibility` (`self.HealthWidget`) false false)
  (`|SpawnActorFromClass` "/Game/MyContent/Interactibles/BP_BossPortal.BP_BossPortal_C" (`KismetMathLibrary.MakeTransform` (33351.0 -9018.0 50.0) (struct :`Yaw` 90.0) (1.5 1.5 1.5)) "AlwaysSpawn" "MultiplyWithRoot" null 0 "Lvl_Office_02" "Office" (`|MakeArray` "Lvl_Boss_01" :!type "Name") null)
  (`KismetSystemLibrary.K2_ClearTimer` null "HandleFaceTarget")
  (`self.OnDeath`))

(fn `HandleFaceTarget`
  (if (and (`self.bFaceTarget`) (not (`self.Attacking`)))
    (bind _targetactor (`self.TargetActor`)
      (:`then`
        (bind (_returnvalue_roll _returnvalue_pitch _returnvalue_yaw) (`KismetMathLibrary.BreakRotator` (`KismetMathLibrary.RInterpTo` (`KismetMathLibrary.FindLookAtRotation` (`self.K2_GetActorLocation`) (`self.K2_GetActorLocation` _targetactor)) (`self.K2_GetActorRotation` _targetactor) (`GameplayStatics.GetWorldDeltaSeconds`) 1.0)))
        (`self.K2_SetActorRotation` (`KismetMathLibrary.MakeRotator` 0.0 0.0 _returnvalue_yaw)))
      (:`else`))))

(fn `InitialiseStats`
  (bind _enemystatcomponent (`self.EnemyStatComponent`))
  (`/Game/MyContent/Core/BP_AC_Stats.SetMaxHealth` _enemystatcomponent (`self.MinMaxHealth`))
  (`self.SetEnemyLevel` (`KismetMathLibrary.FTrunc` (`/Game/MyContent/Core/BP_AC_Stats.Level` _enemystatcomponent)))
  (bind _asbp_uw_enemy_health (cast `/Game/MyContent/Enemies/BP_UW_EnemyHealth` (`WidgetComponent.GetWidget` (`self.HealthWidget`))))
  (`/Game/MyContent/Enemies/BP_UW_EnemyHealth.InitStats` _asbp_uw_enemy_health (`self.EnemyStatComponent`)))

(fn `IsAlive`
  (returns (ReturnValue :type Boolean))
  (return (<= (`/Game/MyContent/Core/BP_AC_Stats.Health` (`self.EnemyStatComponent`)) 0.0)))

(fn `OnTakeDamage`
  (params (DamageCauser :type "Actor Object Reference") (Damage :type "Float (double-precision)"))
  (`/Game/MyContent/Core/BP_AC_Stats.DamageHealth` (`self.EnemyStatComponent`) Damage)
  (if (not (`self.IsAlive`))
    (`self.PlayHitFlash`)
    (`SceneComponent.SetVisibility` (`self.HealthWidget`) true false)
    (else
      (`self.Death`))))

(fn `ResetAttacking`
  (set `self.Attacking` false))

(fn `SetAITarget`
  (params (Target :type "Actor Object Reference")))

(fn `SetEnemyLevel`
  (params (Level :type Integer))
  (bind _enemystatcomponent (`self.EnemyStatComponent`))
  (`/Game/MyContent/Core/BP_AC_Stats.SetLevel` (`self.EnemyStatComponent`) (`KismetMathLibrary.Conv_IntToDouble` Level))
  (`/Game/MyContent/Core/BP_AC_Stats.SetMaxHealth` _enemystatcomponent (* (`/Game/MyContent/Core/BP_AC_Stats.Level` _enemystatcomponent) 100.0))
  (`/Game/MyContent/Core/BP_AC_Stats.SetHealth` _enemystatcomponent (`/Game/MyContent/Core/BP_AC_Stats.MaxHealth` _enemystatcomponent)))

(fn `SetEnemyTarget`
  (params (TargetActor :type "Actor Object Reference"))
  (set `self.TargetActor` TargetActor)
  (bind _assignedcamp (`self.AssignedCamp`)
    (:`then`
      (`/Game/MyContent/Enemies/BP_EnemyCamp.AlertCamp` _assignedcamp self (`self.TargetActor`)))
    (:`else`)))

(fn `SetWeaponOwner`
  (bind _childactor (`ChildActorComponent.ChildActor` (`self.WeaponActorComponent`))
    (:`then`
      (`self.SetOwner` _childactor self))
    (:`else`)))

(fn `SpawnVFX`
  (bind (_returnvalue_location _returnvalue_rotation _returnvalue_scale) (`KismetMathLibrary.BreakTransform` (`self.GetTransform`)))
  (`NiagaraFunctionLibrary.SpawnSystemAtLocation` "/Game/MyContent/VFX/Attacks/NS_Boss_Landing.NS_Boss_Landing" _returnvalue_location _returnvalue_rotation _returnvalue_scale))

(fn `UserConstructionScript`
  (`self.SetWeaponOwner`)
  (`self.CreateDynamicMaterialInstance`))