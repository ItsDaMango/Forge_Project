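; BP_Room is a modular room builder that assembles an office room from static mesh tiles in its construction script, sized by RoomLength and RoomWidth on a 500-unit grid.
; AddFloors creates scene-component row anchors and tiles floors along them, re-looping all anchors per new row, so earlier rows get duplicate meshes.
; AddWalls builds four toggleable sides, each with an optional middle door frame.
; An arrow marks the room centre, hidden at BeginPlay.
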(event `self.ReceiveBeginPlay`
  (`SceneComponent.SetVisibility` (`self.Arrow`) false false))

(fn `AddFloors`
  (for _index (range (`self.RoomLength`))
    (bind _returnvalue (`AddComponent|NODE_AddSceneComponent-1` :`RelativeTransform` (`KismetMathLibrary.MakeTransform` (`KismetMathLibrary.MakeVector` (`KismetMathLibrary.Conv_IntToDouble` (* _index 500))))))
    (`KismetArrayLibrary.Array_Add` (`self.Transforms`) _returnvalue)
    (for _array_element (`self.Transforms`)
      (bind _relativelocation_x (`KismetMathLibrary.BreakVector` (`SceneComponent.RelativeLocation` _array_element)))
      (`self.AddMeshComponent` 0 (`self.RoomWidth`) "/Game/SimpleOffice/Meshes/SM_Floor_01.SM_Floor_01" (`KismetMathLibrary.MakeVector` _relativelocation_x)))))

(fn `AddMeshComponent`
  (params (FirstIndex :type Integer) (LastIndex :type Integer) (NewMesh :type "StaticMesh Object Reference") (Vector :type "Vector Structure" :default (500.0 0.0 0.0)) (`Relative Transform Rotation` :type "Rotator Structure"))
  (for _index (range FirstIndex LastIndex)
    (bind _returnvalue (`AddComponent|NODE_AddStaticMeshComponent-1` :`RelativeTransform` (`KismetMathLibrary.MakeTransform` (`KismetMathLibrary.MakeVector` Vector_X (`KismetMathLibrary.Conv_IntToDouble` (* _index 500)) Vector_Z) `Relative Transform Rotation`)))
    (`StaticMeshComponent.SetStaticMesh` _returnvalue NewMesh)))

(fn `AddWalls`
  (bind _roomwidth (`self.RoomWidth`))
  (bind _roomlength (`self.RoomLength`))
  (bind _transforms (`self.Transforms`))
  (bind _wallmesh (`self.WallMesh`))
  (bind _wallmesh_2 (`self.WallMesh`))
  (bind _wallmesh_3 (`self.WallMesh`))
  (bind (_relativelocation_x _relativelocation_y) (`KismetMathLibrary.BreakVector` (`SceneComponent.RelativeLocation` (`|GetArrayItem` _transforms))))
  (bind (_relativelocation_x_2 _relativelocation_y_2) (`KismetMathLibrary.BreakVector` (`SceneComponent.RelativeLocation` (`|GetArrayItem` _transforms))))
  (bind (_relativelocation_x_3 _relativelocation_y_3) (`KismetMathLibrary.BreakVector` (`SceneComponent.RelativeLocation` (`|GetArrayItem` _transforms))))
  (bind (_relativelocation_x_4 _relativelocation_y_4) (`KismetMathLibrary.BreakVector` (`SceneComponent.RelativeLocation` (`|GetArrayItem` _transforms))))
  (`|ExecutionSequence`
    (:`then_0`
      (if (`self.LeftWall`)
        (for _index (range _roomlength)
          (bind _returnvalue (`AddComponent|NODE_AddStaticMeshComponent-7` :`RelativeTransform` (`KismetMathLibrary.MakeTransform` (`KismetMathLibrary.MakeVector` (`KismetMathLibrary.Conv_IntToDouble` (* _index 500)) _relativelocation_y) (struct))))
          (`StaticMeshComponent.SetStaticMesh` _returnvalue (select `bool` (`self.LeftWallDoor`) :`false` _wallmesh :`true` (select `bool` (== _index (/ _roomlength 2)) :`false` _wallmesh :`true` (`self.DoorFrameMesh`)))))))
    (:`then_1`
      (if (`self.BackWall`)
        (for _index_2 (range _roomwidth)
          (bind _returnvalue_2 (`AddComponent|NODE_AddStaticMeshComponent-6` :`RelativeTransform` (`KismetMathLibrary.MakeTransform` (`KismetMathLibrary.MakeVector` _relativelocation_y_2 (`KismetMathLibrary.Conv_IntToDouble` (* _index_2 500))) (struct :`Yaw` 90.0))))
          (`StaticMeshComponent.SetStaticMesh` _returnvalue_2 (select `bool` (`self.BackWallDoor`) :`false` _wallmesh_3 :`true` (select `bool` (== _index_2 (/ _roomwidth 2)) :`false` _wallmesh_3 :`true` (`self.DoorFrameMesh`)))))))
    (:`then_2`
      (if (`self.RightWall`)
        (for _index_3 (range (`self.RoomLength`))
          (bind _returnvalue_3 (`AddComponent|NODE_AddStaticMeshComponent-8` :`RelativeTransform` (`KismetMathLibrary.MakeTransform` (`KismetMathLibrary.MakeVector` (`KismetMathLibrary.Conv_IntToDouble` (* _index_3 500)) (+ _relativelocation_y_4 (* (`self.RoomWidth`) 500))) (struct))))
          (`StaticMeshComponent.SetStaticMesh` _returnvalue_3 (select `bool` (`self.RightWallDoor`) :`false` _wallmesh_2 :`true` (select `bool` (== (/ (`self.RoomLength`) 2) _index_3) :`false` _wallmesh_2 :`true` (`self.DoorFrameMesh`)))))))
    (:`then_3`
      (if (`self.ForwadWall`)
        (for _index_4 (range (`self.RoomWidth`))
          (bind _returnvalue_4 (`AddComponent|NODE_AddStaticMeshComponent-10` :`RelativeTransform` (`KismetMathLibrary.MakeTransform` (`KismetMathLibrary.MakeVector` (+ _relativelocation_y_3 (* (`self.RoomLength`) 500)) (`KismetMathLibrary.Conv_IntToDouble` (* _index_4 500))) (struct :`Yaw` 90.0))))
          (`StaticMeshComponent.SetStaticMesh` _returnvalue_4 (select `bool` (`self.ForwardWallDoor`) :`false` (`self.WallMesh`) :`true` (select `bool` (== (/ (`self.RoomWidth`) 2) _index_4) :`false` (`self.WallMesh`) :`true` (`self.DoorFrameMesh`)))))))))

(fn `UserConstructionScript`
  (bind _returnvalue_location (`KismetMathLibrary.BreakTransform` (`SceneComponent.GetRelativeTransform` (`self.Root`))))
  (bind (_returnvalue_x _returnvalue_y _returnvalue_z) (`KismetMathLibrary.BreakVector` (+ _returnvalue_location (`KismetMathLibrary.MakeVector` (/ (* (`self.RoomLength`) 500) 2) (/ (* (`self.RoomWidth`) 500) 2) 300.0))))
  (`KismetArrayLibrary.Array_Clear` (`self.Transforms`))
  (`self.AddFloors`)
  (`self.AddWalls`)
  (`SceneComponent.K2_SetRelativeLocation` (`self.Arrow`) (`KismetMathLibrary.MakeVector` _returnvalue_x _returnvalue_y _returnvalue_z) false false))