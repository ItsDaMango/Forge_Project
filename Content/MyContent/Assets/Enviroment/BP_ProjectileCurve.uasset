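; BP_ProjectileCurve is an actor meant to travel an arced path between a start and an end location.
; The Initial event stores both endpoints.
; Tick lerps between them by elapsed time over Time, adding a sine offset along the actor's up vector scaled by Height.
; The destroy check compares elapsed time to zero rather than Time, so as written the actor is destroyed on its first tick.
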(event `self.ReceiveTick`
  (params (DeltaSeconds :type "Float (single-precision)"))
  (bind _output_get (set `self.Elapsed` (+ DeltaSeconds (`self.Elapsed`))))
  (bind _output_get_2 (set `self.Alpha` (/ _output_get (`self.Time`))))
  (`self.K2_SetActorLocation` (+ (* (`self.GetActorUpVector`) (* (`KismetMathLibrary.Sin` (`KismetMathLibrary.MultiplyByPi` _output_get_2)) (`self.Height`))) (`KismetMathLibrary.VLerp` (`self.StartLocation`) (`self.EndLocation`) (`self.Alpha`))))
  (if (>= (`self.Elapsed`) 0.0)
    (`self.K2_DestroyActor`)))

(event `Initial`
  (params (StartLocation :type "Vector Structure") (EndLocation :type "Vector Structure"))
  (set `self.StartLocation` StartLocation)
  (set `self.EndLocation` EndLocation))

(fn `UserConstructionScript`)