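; BP_ProjectileSpawner is an environment actor that repeatedly fires curved projectiles at the player.
; After a short delay on BeginPlay, a looping timer spawns a BP_ProjectileCurve at the SpawnLocation component.
; Each projectile is initialized with that start point and the player pawn's position at spawn time as its end point, so it does not receive later position updates from the spawner.
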(event `self.ReceiveBeginPlay`
  (`KismetSystemLibrary.Delay` 2.0)
  (`KismetSystemLibrary.K2_SetTimerDelegate` (delegate `Spawn`) 1.0 true))

(event `Spawn`
  (bind _returnvalue (`|SpawnActorFromClass` "/Game/MyContent/Assets/Enviroment/BP_ProjectileCurve.BP_ProjectileCurve_C" (`KismetMathLibrary.MakeTransform` (`SceneComponent.K2_GetComponentLocation` (`self.SpawnLocation`))) "Undefined" "MultiplyWithRoot" null null))
  (`/Game/MyContent/Assets/Enviroment/BP_ProjectileCurve.Initial` _returnvalue (`SceneComponent.K2_GetComponentLocation` (`self.SpawnLocation`)) (`self.K2_GetActorLocation` (`GameplayStatics.GetPlayerPawn` 0))))

(fn `UserConstructionScript`)