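; Boss-fight variant of a roller log trap, tied to BP_Boss1 and its death event.
; BeginPlay creates a dynamic indicator material, binds to the boss's OnDeath, then after a delay calls SetLogTrap and starts a fast looping timer.
; Tick feeds Alpha into the indicator material, and TurnOff calls Stop.
; The parent BeginPlay is never run, so this setup replaces it.
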(event `self.ReceiveBeginPlay`
  (bind _returnvalue (`DecalComponent.CreateDynamicMaterialInstance` (`self.Indicator`)))
  (set `self.Indicater_MI` _returnvalue)
  (bind _returnvalue_2 (`GameplayStatics.GetActorOfClass` "/Game/MyContent/Boss/BP_Boss1.BP_Boss1_C"))
  (bind _output_get (set `self.BossRef` _returnvalue_2))
  (add `/Game/MyContent/Boss/BP_Boss1.OnDeath` _output_get (`|CreateDelegate` :!event `TurnOff`))
  (`KismetSystemLibrary.Delay` 4.0)
  (`self.SetLogTrap`)
  (`KismetSystemLibrary.K2_SetTimerDelegate` (`|CreateDelegate` :!event `Roll`) 0.01 true))

(event `self.ReceiveTick`
  (params (DeltaSeconds :type "Float (single-precision)"))
  (`parent.ReceiveTick` DeltaSeconds)
  (`MaterialInstanceDynamic.SetScalarParameterValue` (`self.Indicater_MI`) "Alpha" (`self.Alpha`)))

(event `TurnOff`
  (`self.Stop`))

(fn `UserConstructionScript`
  (`parent.UserConstructionScript`))