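; BP_SwingingAxe is a trap prop with a swinging axe that damages the player on contact.
; On BeginPlay, the AxeSwing timeline drives the axe's relative pitch, with a DoOnce playing the axe sound at the actor's location on the first update, reset when the timeline finishes.
; An overlap with BP_PlayerCharacter applies fixed damage, then after a short delay briefly disables the axe's collision before restoring it to query-only.
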(event `self.ReceiveBeginPlay`
  (bind (_direction _axe_swinging) (`Timeline|Axe Swing`)
    (:`Update`
      (`SceneComponent.K2_SetRelativeRotation` (`self.Axe`) (`KismetMathLibrary.MakeRotator` 0.0 _axe_swinging) false false)
      (`/Engine/EditorBlueprintResources/StandardMacros.DoOnce` false :!label _label
        (:`Completed`
          (bind _returnvalue (`GameplayStatics.SpawnSoundAtLocation` "/Game/MyContent/SFX/SC_Axe.SC_Axe" (`self.K2_GetActorLocation`) (struct) 1.0 1.0 0.0 "/Game/MyContent/SFX/SA_Default.SA_Default" null))
          (`AudioComponent.Play` _returnvalue 0.0))))
    (:`Finished`
      (goto _label :!via `Reset`))))

(event `self.Axe.OnComponentBeginOverlap`
  (params (OverlappedComponent :type "PrimitiveComponent Object Reference") (OtherActor :type "Actor Object Reference") (OtherComp :type "PrimitiveComponent Object Reference") (OtherBodyIndex :type Integer) (bFromSweep :type Boolean) (SweepResult :type "HitResult Structure (by ref)"))
  (bind _asbp_player_character (cast `/Game/MyContent/Player/BP_PlayerCharacter` OtherActor))
  (`GameplayStatics.ApplyDamage` _asbp_player_character 15.0)
  (`KismetSystemLibrary.Delay` 1.0)
  (`PrimitiveComponent.SetCollisionEnabled` (`self.Axe`) "NoCollision")
  (`KismetSystemLibrary.Delay` 1.0)
  (`PrimitiveComponent.SetCollisionEnabled` (`self.Axe`) "QueryOnly"))

(fn `UserConstructionScript`)