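; BP_Roller is a rolling log trap that repeatedly travels from a start point to an end point, damaging the player on contact.
; After a random delay, it plays a sound and runs a timeline lerp, restarting itself while Active.
; A Roll event spins the mesh at a periodically randomized speed.
; Capsule overlaps apply damage, then briefly disable mesh collision as a hit cooldown.
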(event `self.ReceiveBeginPlay`
  (`self.SetLogTrap`)
  (bind _asbp_game_instance (cast `/Game/MyContent/Core/BP_GameInstance` (`GameplayStatics.GetGameInstance`)))
  (`KismetSystemLibrary.K2_SetTimerDelegate` (`|CreateDelegate` :!event `Roll`) 0.01 true)
  (set `self.RollSpeed` (`KismetMathLibrary.RandomFloatInRange` 5.0 15.0)))

(event `Reverse`
  (bind _randomoffset (`self.RandomOffset`))
  (`KismetSystemLibrary.Delay` (`KismetMathLibrary.RandomFloatInRange` (- _randomoffset 1.0) (+ _randomoffset 5.0)) :!label _label)
  (bind _returnvalue (`GameplayStatics.SpawnSoundAtLocation` (`self.SoundCue`) (`self.K2_GetActorLocation`) (struct) 1.0 1.0 0.0 null null))
  (`AudioComponent.Play` _returnvalue 0.0)
  (bind (_direction _alpha_5s _alpha_3s) (`Timeline|TL_Log` :!via `PlayFromStart`)
    (:`Update`
      (set `self.Alpha` _alpha_5s)
      (bind _output_get (set `self.Vector` (`KismetMathLibrary.VLerp` (`SceneComponent.K2_GetComponentLocation` (`self.Start`)) (`SceneComponent.K2_GetComponentLocation` (`self.End`)) _alpha_3s)))
      (`SceneComponent.K2_SetWorldLocation` (`self.Mesh`) _output_get false false))
    (:`Finished`
      (if (`self.Active`)
        (`self.Reverse`)))))

(event `SetLogTrap`
  (goto _label))

(event `self.ReceiveTick`
  (params (DeltaSeconds :type "Float (single-precision)")))

(event `Stop`
  (set `self.Active` false))

(event `Roll`
  (bind _mesh (`self.Mesh`))
  (bind (_relativerotation_roll _relativerotation_pitch _relativerotation_yaw) (`KismetMathLibrary.BreakRotator` (`SceneComponent.RelativeRotation` _mesh)))
  (`|ExecutionSequence`
    (:`then_0`
      (`SceneComponent.K2_SetRelativeRotation` _mesh (`KismetMathLibrary.MakeRotator` 90.0 0.0 (+ _relativerotation_yaw (`self.RollSpeed`))) false false))
    (:`then_1`
      (`KismetSystemLibrary.Delay` 4.0)
      (set `self.RollSpeed` (`KismetMathLibrary.RandomFloatInRange` 3.0 15.0)))))

(event `self.Mesh.OnComponentBeginOverlap`
  (params (OverlappedComponent :type "PrimitiveComponent Object Reference") (OtherActor :type "Actor Object Reference") (OtherComp :type "PrimitiveComponent Object Reference") (OtherBodyIndex :type Integer) (bFromSweep :type Boolean) (SweepResult :type "HitResult Structure (by ref)"))
  (bind _asbp_player_character (cast `/Game/MyContent/Player/BP_PlayerCharacter` OtherActor))
  (if (== OtherComp (`Character.CapsuleComponent` _asbp_player_character))
    (`GameplayStatics.ApplyDamage` OtherActor (`self.Damage`) null self)
    (`PrimitiveComponent.SetCollisionEnabled` (`self.Mesh`) "NoCollision")
    (`KismetSystemLibrary.Delay` (`self.DamageDelay`))
    (`PrimitiveComponent.SetCollisionEnabled` (`self.Mesh`) "QueryOnly")))

(fn `UserConstructionScript`)