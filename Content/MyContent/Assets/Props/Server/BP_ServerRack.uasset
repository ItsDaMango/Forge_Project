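; Server rack prop that shows a randomly coloured, continuously animated glow on its static mesh.
; The construction script creates a dynamic material instance, and BeginPlay gives it a random colour and picks a random multiplier.
; A self-restarting timeline drives the glow strength, multiplying its alpha by that multiplier before the Lerp, so each rack's intensity varies.
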(event `self.ReceiveBeginPlay`
  (`self.AlphaGlow`)
  (set `self.Random` (`KismetMathLibrary.RandomFloatInRange` 1.0 200.0))
  (`MaterialInstanceDynamic.SetVectorParameterValue` (`self.ServerMI`) "Colour" (make `LinearColor` (`KismetMathLibrary.RandomFloat`) (`KismetMathLibrary.RandomFloat`) (`KismetMathLibrary.RandomFloat`) 1.0)))

(event `AlphaGlow`
  (bind (_direction _alpha) (`Timeline|TL_GlowAlpha` :!via `PlayFromStart`)
    (:`Update`
      (`MaterialInstanceDynamic.SetScalarParameterValue` (`self.ServerMI`) "Strength" (`KismetMathLibrary.Lerp` 0.5 20.0 (* _alpha (`self.Random`)))))
    (:`Finished`
      (`self.AlphaGlow`))))

(fn `UserConstructionScript`
  (bind _staticmesh (`self.StaticMesh`))
  (bind _returnvalue (`PrimitiveComponent.CreateDynamicMaterialInstance` _staticmesh 0 (`PrimitiveComponent.GetMaterial` _staticmesh 0) "None"))
  (set `self.ServerMI` _returnvalue))