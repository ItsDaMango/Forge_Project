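; BP_Pickup_SkillPoint is a child pickup that grants the player one skill point when collected.
; OnPickup runs the parent logic, then increments the player's SkillPoints and updates the HUD text through BP_GM_Main.
; An overlay-material effect driven by a timeline alpha is left disconnected: the material setup and its looping timer never run.
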(event `self.ReceiveBeginPlay`
  (`parent.ReceiveBeginPlay`))

(event `OverlayAlpha`
  (`MaterialInstanceDynamic.SetScalarParameterValue` (`self.OverlayMI`) "Strength" (/ (`self.TimelineAlpha`) 1.0)))

(fn `OnPickup`
  (params (PlayerRef :type "/Game/MyContent/Player/BP_PlayerCharacter Object Reference"))
  (`parent.OnPickup` PlayerRef)
  (bind _asbp_gm_main (cast `/Game/MyContent/Core/BP_GM_Main` (`GameplayStatics.GetGameMode`)))
  (bind _result (`/Engine/EditorBlueprintResources/StandardMacros.IncrementInt` (`/Game/MyContent/Player/BP_PlayerCharacter.SkillPoints` PlayerRef))
    (:`  `
      (`/Game/MyContent/Player/HUD/BP_UI_HUD.SetSkillPointText` (`/Game/MyContent/Core/BP_GM_Main.GM_HUD` _asbp_gm_main) _result))))

(fn `UserConstructionScript`
  (`parent.UserConstructionScript`))