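; BP_Pickup is an item pickup that bobs and spins until a living BP_PlayerCharacter collects it.
; A self-restarting timeline offsets its height, and Tick adds a fixed yaw each frame, independent of delta time.
; When the player's capsule overlaps PickupCollision, it calls OnPickup with the player, then hides the root and skeletal mesh without destroying the actor.
; OnPickup itself only clears AllowPickup, blocking repeat collection.
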(event `MovePickup`
  (set `self.ActorLoc` (`self.K2_GetActorLocation`))
  (bind (_direction _alpha) (`Timeline|TL_OffsetPickup` :!via `PlayFromStart`)
    (:`Update`
      (bind _output_get (set `self.TimelineAlpha` _alpha))
      (`self.K2_SetActorLocation` (`KismetMathLibrary.VLerp` (`self.ActorLoc`) (+ (`self.ActorLoc`) (0.0 0.0 15.0)) _output_get)))
    (:`Finished`
      (`self.MovePickup`))))

(event `self.ReceiveBeginPlay`
  (`parent.ReceiveBeginPlay`)
  (`self.MovePickup`))

(event `self.ReceiveTick`
  (params (DeltaSeconds :type "Float (single-precision)"))
  (`parent.ReceiveTick` DeltaSeconds)
  (`self.Rotate`))

(event `self.PickupCollision.OnComponentBeginOverlap`
  (params (OverlappedComponent :type "PrimitiveComponent Object Reference") (OtherActor :type "Actor Object Reference") (OtherComp :type "PrimitiveComponent Object Reference") (OtherBodyIndex :type Integer) (bFromSweep :type Boolean) (SweepResult :type "HitResult Structure (by ref)"))
  (bind _asbp_player_character (cast `/Game/MyContent/Player/BP_PlayerCharacter` OtherActor))
  (if (and (`self.bAllowPickup`) (`/Game/MyContent/Core/BP_AC_Stats.IsAlive` (`/Game/MyContent/Player/BP_PlayerCharacter.StatComponent` _asbp_player_character)) (== OtherComp (`Character.CapsuleComponent` _asbp_player_character)))
    (`self.OnPickup` _asbp_player_character)
    (`SceneComponent.SetVisibility` (`self.DefaultSceneRoot`) false false)
    (`SceneComponent.SetVisibility` (`self.SkeletalMesh`) false false)))

(fn `OnPickup`
  (params (PlayerRef :type "/Game/MyContent/Player/BP_PlayerCharacter Object Reference"))
  (set `self.bAllowPickup` false))

(fn `Rotate`
  (`self.K2_AddActorLocalRotation` (struct :`Yaw` 2.0)))

(fn `UserConstructionScript`
  (`parent.UserConstructionScript`))