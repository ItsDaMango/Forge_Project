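; Regular health pickup Blueprint that heals the player who collects it.
; It overrides the parent's OnPickup, calls the parent logic, then applies HealAmount through the player's StatComponent.
; It also deactivates the NSHeal effect, zeroes that effect's particle lifetime parameters and plays a 2D sound.
; BeginPlay, Tick and construction only forward to the parent, and the overlap event is disabled.
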(event `self.ReceiveBeginPlay`
  (`parent.ReceiveBeginPlay`))

(event `self.ReceiveTick`
  (params (DeltaSeconds :type "Float (single-precision)"))
  (`parent.ReceiveTick` DeltaSeconds))

(fn `OnPickup`
  (params (PlayerRef :type "/Game/MyContent/Player/BP_PlayerCharacter Object Reference"))
  (bind _ns_heal (`self.NS_Heal`))
  (`parent.OnPickup` PlayerRef)
  (`ActorComponent.Deactivate` _ns_heal)
  (`/Game/MyContent/Core/BP_AC_Stats.HealHealth` (`/Game/MyContent/Player/BP_PlayerCharacter.StatComponent` (`local.PlayerRef`)) (`self.HealAmount`))
  (`FXSystemComponent.SetFloatParameter` _ns_heal "P_LifetimeMax" 0.0)
  (`FXSystemComponent.SetFloatParameter` _ns_heal "P_LifetimeMin" 0.0)
  (`GameplayStatics.PlaySound2D` "/Engine/VREditor/Sounds/UI/Enter_Play.Enter_Play" 1.0 1.0 0.0 null null))

(fn `UserConstructionScript`
  (`parent.UserConstructionScript`))