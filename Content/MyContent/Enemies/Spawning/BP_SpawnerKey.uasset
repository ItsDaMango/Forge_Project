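; BP_SpawnerKey is a damageable key actor that counts toward a spawn point's collected keys when destroyed.
; A randomized looping timer and the PlayAlphaFlash event's FlipFlop timeline pulse a parameter on the mesh's dynamic material.
; Damage feeds HealthComponent; on death it clears the flash timer, increments KeysCollected on SpawnPoint, prints the result and destroys itself.
; CheckKeys and the construction script are empty.
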(event `self.ReceiveBeginPlay`
  (bind _returnvalue (`PrimitiveComponent.CreateDynamicMaterialInstance` (`self.SM_DeskPreset_02`) 0 (`PrimitiveComponent.GetMaterial` (`self.SM_DeskPreset_02`) 0) "None"))
  (set `self.MeshMaterialDynamic` _returnvalue)
  (`KismetSystemLibrary.K2_SetTimerDelegate` (`|CreateDelegate` :!event `PlayAlphaFlash`) (`KismetMathLibrary.RandomFloatInRange` 1.0 2.0) true)
  (`MaterialInstanceDynamic.SetScalarParameterValue` (`self.MeshMaterialDynamic`) "EmissiveStrength" 0.2))

(event `PlayAlphaFlash`
  (`/Engine/EditorBlueprintResources/StandardMacros.FlipFlop`
    (:`A`
      (bind (_direction _alpha) (`Timeline|AlphaFlash` :!label _label)
        (:`Update`
          (`MaterialInstanceDynamic.SetScalarParameterValue` (`self.MeshMaterialDynamic`) "AlphaFlash" (* _alpha 0.1)))))
    (:`B`
      (goto _label :!via `Reverse`))))

(event `self.ReceiveAnyDamage`
  (params (Damage :type "Float (single-precision)") (DamageType :type "DamageType Object Reference") (InstigatedBy :type "Controller Object Reference") (DamageCauser :type "Actor Object Reference"))
  (bind _healthcomponent (`self.HealthComponent`))
  (`/Game/MyContent/Core/BP_AC_Stats.DamageHealth` _healthcomponent Damage)
  (if (not (`/Game/MyContent/Core/BP_AC_Stats.IsAlive` _healthcomponent))
    (`KismetSystemLibrary.K2_ClearTimer` null "PlayAlphaFlash")
    (bind _currentcount (`self.AddKey`))
    (`KismetSystemLibrary.PrintString` (`KismetStringLibrary.Conv_IntToString` _currentcount))
    (`self.K2_DestroyActor`)))

(fn `AddKey`
  (returns (CurrentCount :type Integer))
  (bind _result (`/Engine/EditorBlueprintResources/StandardMacros.IncrementInt` (`/Game/MyContent/Enemies/Spawning/BP_SpawnPoint.KeysCollected` (`self.SpawnPoint`)))
    (:`  `
      (return _result))))

(fn `CheckKeys`)

(fn `UserConstructionScript`)