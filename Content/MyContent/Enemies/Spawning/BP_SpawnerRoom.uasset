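; BP_SpawnerRoom is a room trigger that spawns enemies when the player enters.
; Its SpawnCollision overlap checks for BP_PlayerCharacter, then sets a half-second timer and an IsTriggered flag so it fires only once.
; SpawnEnemies, the apparent timer target, loops over SpawnPoints and calls SpawnEnemy on each valid one.
; EnemiesToSpawn is left unused, so each spawn point gets one call.
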(event `self.ReceiveBeginPlay`)

(event `self.SpawnCollision.OnComponentBeginOverlap`
  (params (OverlappedComponent :type "PrimitiveComponent Object Reference") (OtherActor :type "Actor Object Reference") (OtherComp :type "PrimitiveComponent Object Reference") (OtherBodyIndex :type Integer) (bFromSweep :type Boolean) (SweepResult :type "HitResult Structure (by ref)"))
  (cast `/Game/MyContent/Player/BP_PlayerCharacter` OtherActor)
  (if (not (`self.bIsTriggered`))
    (`KismetSystemLibrary.K2_SetTimerDelegate` (`|CreateDelegate` :!event `SpawnEnemies`) 0.5)
    (set `self.bIsTriggered` true)))

(event `SpawnEnemies`
  (bind _spawnpoints (`self.SpawnPoints`))
  (if (`KismetArrayLibrary.Array_IsNotEmpty` _spawnpoints)
    (for _index (range (+ (`KismetArrayLibrary.Array_Length` _spawnpoints) 1))
      (bind _output (`|GetArrayItem` _spawnpoints _index))
      (`/Engine/EditorBlueprintResources/StandardMacros.IsValid` _output
        (:`Is Valid`
          (`/Game/MyContent/Enemies/Spawning/BP_SpawnPoint.SpawnEnemy` _output))))))

(fn `UserConstructionScript`)