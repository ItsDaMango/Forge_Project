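; Enemy spawn point that repeatedly spawns an enemy every 2–5 seconds, paced by a Delay on Tick, until the MaxSpawns limit is passed (zero means unlimited).
; Each spawn flashes the cone material, plays a Niagara portal at a randomly offset position, then spawns the enemy and assigns melee enemies to EnemyCamp.
; Spawn attempts also check the key count, messaging DoorRef and destroying the spawner once enough keys are collected.
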(event `self.ReceiveBeginPlay`
  (bind _cone (`self.Cone`))
  (bind _returnvalue (`PrimitiveComponent.CreateDynamicMaterialInstance` _cone 0 (`PrimitiveComponent.GetMaterial` _cone 0) "None"))
  (set `self.ConeMaterial` _returnvalue))

(event `self.ReceiveTick`
  (params (DeltaSeconds :type "Float (single-precision)"))
  (`KismetSystemLibrary.Delay` (`KismetMathLibrary.RandomFloatInRange` 2.0 5.0))
  (if (or (>= (`self.MaxSpawns`) (`self.Spawns`)) (== (`self.MaxSpawns`) 0))
    (`self.SpawnEnemy`)
    (else
      (`MaterialInstanceDynamic.SetScalarParameterValue` (`self.ConeMaterial`) "Intensity" 0.0))))

(event `SpawnEnemy`
  (bind (_localtransform_x _localtransform_y _localtransform_z) (`KismetMathLibrary.BreakVector` (`self.LocalTransform`)))
  (bind _returnvalue (`SceneComponent.K2_GetComponentLocation` (`self.EnemySpawnTransform`)))
  (bind (_returnvalue_location _returnvalue_rotation _returnvalue_scale) (`KismetMathLibrary.BreakTransform` (`SceneComponent.K2_GetComponentToWorld` (`self.EnemySpawnTransform`))))
  (`/Engine/EditorBlueprintResources/StandardMacros.IncrementInt` (`self.Spawns`)
    (:`  `
      (`MaterialInstanceDynamic.SetScalarParameterValue` (`self.ConeMaterial`) "Intensity" 400.0)
      (`self.KeyCount`)
      (if (`KismetSystemLibrary.IsValid` self)
        (set `self.LocalTransform` (+ _returnvalue (`KismetMathLibrary.MakeVector` (`KismetMathLibrary.RandomFloatInRange` -100.0 100.0) (`KismetMathLibrary.RandomFloatInRange` -100.0 100.0) (.z _returnvalue))))
        (bind _returnvalue_2 (`NiagaraFunctionLibrary.SpawnSystemAtLocation` "/Game/MyContent/VFX/Portals/NS_BasicPortal_V2.NS_BasicPortal_V2" (`KismetMathLibrary.MakeVector` _localtransform_x _localtransform_y (- _localtransform_z 65.0)) (struct :`Yaw` 90.0) (0.4 0.4 1.0) true true "AutoRelease"))
        (`ActorComponent.Activate` _returnvalue_2 true)
        (`|ExecutionSequence`
          (:`then_0`
            (`MaterialInstanceDynamic.SetScalarParameterValue` (`self.ConeMaterial`) "Intensity" 10.0))
          (:`then_1`
            (`KismetSystemLibrary.Delay` 0.2)
            (bind _returnvalue_3 (`|SpawnActorFromClass` (`self.Enemy`) (`KismetMathLibrary.MakeTransform` (`self.LocalTransform`) _returnvalue_rotation _returnvalue_scale) "AdjustIfPossibleButAlwaysSpawn" "MultiplyWithRoot" null null))
            (bind _asbp_enemy_melee (cast `/Game/MyContent/Enemies/BP_Enemy_Melee` _returnvalue_3))
            (bind _enemycamp (`self.EnemyCamp`)
              (:`then`
                (set `/Game/MyContent/Enemies/BP_Enemy.AssignedCamp` _enemycamp _asbp_enemy_melee))
              (:`else`))))))))

(fn `IsInteractable`
  (returns (Interactable :type Boolean))
  (return false))

(fn `KeyCount`
  (if (>= (`self.KeysCollected`) (`self.KeysNeeded`))
    (message `/Game/MyContent/Interface/BPI_InteractInterface.OnInteract` (`self.DoorRef`) null)
    (`self.K2_DestroyActor`)))

(fn `UserConstructionScript`)