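; Melee enemy Blueprint that specialises a parent enemy class with a hammer weapon and its own health bar colour.
; On possession, after a short delay, it tints the health widget's bar purple and then sets the damage on the BP_NokiaHammer child actor.
; BeginPlay, construction and SetEnemyTarget only call the parent; a walk-speed change in SetEnemyTarget is disconnected and never runs.
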(event `self.ReceivePossessed`
  (params (NewController :type "Controller Object Reference"))
  (`parent.ReceivePossessed` NewController)
  (`KismetSystemLibrary.Delay` 0.1)
  (bind _asbp_uw_enemy_health (cast `/Game/MyContent/Enemies/BP_UW_EnemyHealth` (`WidgetComponent.GetWidget` (`self.HealthWidget`))))
  (set `/Game/MyContent/Enemies/BP_UW_EnemyHealth.HPBarColour` (struct :`R` 0.450976 :`B` 1.0 :`A` 1.0) _asbp_uw_enemy_health)
  (`/Game/MyContent/Enemies/BP_UW_EnemyHealth.SetBarColour` _asbp_uw_enemy_health)
  (bind _asbp_nokia_hammer (cast `/Game/MyContent/Weapons/BP_NokiaHammer` (`ChildActorComponent.ChildActor` (`self.WeaponActorComponent`))))
  (set `/Game/MyContent/Weapons/BP_Weapon.Damage` 15.0 _asbp_nokia_hammer))

(event `self.ReceiveBeginPlay`
  (`parent.ReceiveBeginPlay`))

(fn `SetEnemyTarget`
  (params (TargetActor :type "Actor Object Reference"))
  (`parent.SetEnemyTarget` TargetActor))

(fn `UserConstructionScript`
  (`parent.UserConstructionScript`))