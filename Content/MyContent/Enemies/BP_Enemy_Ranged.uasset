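; Ranged enemy variant that attacks by throwing spears, extending a parent enemy class.
; BeginPlay swaps the attack montage list for a single ranged montage and sets a long attack range.
; Attack runs the parent logic, faces the target, then spawns a spear weapon actor at the enemy's own transform.
; Unconnected trace and direct-damage nodes remain in the Attack graph but never run.
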(event `self.ReceiveBeginPlay`
  (`parent.ReceiveBeginPlay`)
  (`KismetArrayLibrary.Array_Clear` (`self.AttackAnims`))
  (`KismetArrayLibrary.Array_Add` (`self.AttackAnims`) "/Game/PolyHP_Goblin/Animations/ms05_04_Attack_04_Ranged_Montage.ms05_04_Attack_04_Ranged_Montage")
  (set `self.AttackRange` 1500.0))

(fn `Attack`
  (returns (ReturnValue :type "Float (single-precision)"))
  (`parent.Attack`)
  (`self.HandleFaceTarget`)
  (`|SpawnActorFromClass` "/Game/MyContent/Weapons/BP_WeaponSpear.BP_WeaponSpear_C" (`self.GetTransform`) "AlwaysSpawn" "MultiplyWithRoot" null null))

(fn `UserConstructionScript`
  (`parent.UserConstructionScript`))