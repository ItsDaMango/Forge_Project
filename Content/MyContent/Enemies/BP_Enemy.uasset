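; Base enemy character with a child-actor weapon, level-scaled health, health widget and camp membership that alerts the camp when it gets a target.
; Damage plays a hit reaction and timeline-driven dynamic-material flash, or triggers death, which drops a health pickup and disables weapon damage.
; Attack plays a random montage, and Tick handles optional target facing.
; IsAlive is inverted, returning true at zero health or below, and OnTakeDamage branches accordingly.
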(event `self.ReceiveBeginPlay`
  (`|ExecutionSequence`
    (:`then_0`
      (`self.InitialiseStats`)
      (bind _asbp_weapon (cast `/Game/MyContent/Weapons/BP_Weapon` (`ChildActorComponent.ChildActor` (`self.WeaponActorComponent`))))
      (set `/Game/MyContent/Weapons/BP_Weapon.ClassToIgnore` (`self.Classes to IgnoreDamge`) _asbp_weapon))
    (:`then_1`
      (bind _assignedcamp (`self.AssignedCamp`)
        (:`then`
          (`/Game/MyContent/Enemies/BP_EnemyCamp.AddEnemies` _assignedcamp self))
        (:`else`)))))

(event `PlayHitFlash`
  (bind (_direction _alpha) (`Timeline|TL_HitFlash` :!via `PlayFromStart`)
    (:`Update`
      (for _array_element (`self.MeshMaterials`)
        (`MaterialInstanceDynamic.SetScalarParameterValue` _array_element "HitFlashAlpha" _alpha)))))

(event `self.ReceiveTick`
  (params (DeltaSeconds :type "Float (single-precision)"))
  (`self.HandleFaceTarget`))

(event `self.ReceiveAnyDamage`
  (params (Damage :type "Float (single-precision)") (DamageType :type "DamageType Object Reference") (InstigatedBy :type "Controller Object Reference") (DamageCauser :type "Actor Object Reference"))
  (`self.OnTakeDamage` DamageCauser Damage))

(fn `ActivateDamage`
  (bind _asbp_weapon (cast `/Game/MyContent/Weapons/BP_Weapon` (`ChildActorComponent.ChildActor` (`self.WeaponActorComponent`))))
  (`/Game/MyContent/Weapons/BP_Weapon.ActivateDamage` _asbp_weapon))

(fn `Attack`
  (returns (ReturnValue :type "Float (single-precision)"))
  (if (`KismetArrayLibrary.Array_IsNotEmpty` (`self.AttackAnims`))
    (bind _returnvalue (`AnimInstance.Montage_Play` (`SkeletalMeshComponent.GetAnimInstance` (`self.Mesh`)) (`KismetArrayLibrary.Array_Random` (`self.AttackAnims`)) 1.0 "Duration" 0.0 true))
    (return _returnvalue)))

(fn `CreateDynamicMaterialInstance`
  (`KismetArrayLibrary.Array_Clear` (`self.MeshMaterials`))
  (for (_array_element _array_index) (`MeshComponent.GetMaterials` (`self.Mesh`))
    (bind _returnvalue (`PrimitiveComponent.CreateDynamicMaterialInstance` (`self.Mesh`) _array_index _array_element "None"))
    (`KismetArrayLibrary.Array_Add` (`self.MeshMaterials`) _returnvalue)))

(fn `DeactivateDamage`
  (bind _asbp_weapon (cast `/Game/MyContent/Weapons/BP_Weapon` (`ChildActorComponent.ChildActor` (`self.WeaponActorComponent`))))
  (`/Game/MyContent/Weapons/BP_Weapon.DeactivateDamage` _asbp_weapon))

(fn `Death`
  (bind _returnvalue_location (`KismetMathLibrary.BreakTransform` (`self.GetTransform`)))
  (set `self.bCanBeDamaged` false)
  (`PrimitiveComponent.SetCollisionResponseToChannel` (`self.CapsuleComponent`) "ECC_Pawn" "ECR_Ignore")
  (`PrimitiveComponent.SetCollisionEnabled` (`self.Mesh`) "PhysicsOnly")
  (`SceneComponent.SetVisibility` (`self.HealthWidget`) false false)
  (`|SpawnActorFromClass` "/Game/MyContent/Items/BP_Pickup_Health_Regular.BP_Pickup_Health_Regular_C" (`KismetMathLibrary.MakeTransform` (- _returnvalue_location (0.0 0.0 70.0))) "Undefined" "MultiplyWithRoot" null 20.0 null)
  (`self.OnDeath`)
  (`self.DeactivateDamage`))

(fn `HandleFaceTarget`
  (if (`self.bFaceTarget`)
    (bind _targetactor (`self.TargetActor`)
      (:`then`
        (bind (_returnvalue_roll _returnvalue_pitch _returnvalue_yaw) (`KismetMathLibrary.BreakRotator` (`KismetMathLibrary.RInterpTo` (`KismetMathLibrary.FindLookAtRotation` (`self.K2_GetActorLocation`) (`self.K2_GetActorLocation` _targetactor)) (struct) (`GameplayStatics.GetWorldDeltaSeconds`) 10.0)))
        (`self.K2_SetActorRotation` (`KismetMathLibrary.MakeRotator` 0.0 0.0 _returnvalue_yaw)))
      (:`else`))))

(fn `InitialiseStats`
  (`self.SetEnemyLevel` (`KismetMathLibrary.FTrunc` (`/Game/MyContent/Core/BP_AC_Stats.Level` (`self.EnemyStatComponent`))))
  (bind _asbp_uw_enemy_health (cast `/Game/MyContent/Enemies/BP_UW_EnemyHealth` (`WidgetComponent.GetWidget` (`self.HealthWidget`))))
  (`/Game/MyContent/Enemies/BP_UW_EnemyHealth.InitialiseHealth` _asbp_uw_enemy_health (`self.EnemyStatComponent`)))

(fn `IsAlive`
  (returns (ReturnValue :type Boolean))
  (return (<= (`/Game/MyContent/Core/BP_AC_Stats.Health` (`self.EnemyStatComponent`)) 0.0)))

(fn `OnTakeDamage`
  (params (DamageCauser :type "Actor Object Reference") (Damage :type "Float (double-precision)"))
  (`/Game/MyContent/Core/BP_AC_Stats.DamageHealth` (`self.EnemyStatComponent`) Damage)
  (if (not (`self.IsAlive`))
    (`self.PlayAnimMontage` (`self.HitReactAnim`))
    (`self.PlayHitFlash`)
    (`SceneComponent.SetVisibility` (`self.HealthWidget`) true false)
    (else
      (`self.Death`))))

(fn `SetAITarget`
  (params (Target :type "Actor Object Reference")))

(fn `SetEnemyLevel`
  (params (Level :type Integer))
  (bind _enemystatcomponent (`self.EnemyStatComponent`))
  (`/Game/MyContent/Core/BP_AC_Stats.SetLevel` (`self.EnemyStatComponent`) (`KismetMathLibrary.Conv_IntToDouble` Level))
  (`/Game/MyContent/Core/BP_AC_Stats.SetMaxHealth` _enemystatcomponent (* (`/Game/MyContent/Core/BP_AC_Stats.Level` _enemystatcomponent) 100.0))
  (`/Game/MyContent/Core/BP_AC_Stats.SetHealth` _enemystatcomponent (`/Game/MyContent/Core/BP_AC_Stats.MaxHealth` _enemystatcomponent)))

(fn `SetEnemyTarget`
  (params (TargetActor :type "Actor Object Reference"))
  (set `self.TargetActor` TargetActor)
  (bind _assignedcamp (`self.AssignedCamp`)
    (:`then`
      (`/Game/MyContent/Enemies/BP_EnemyCamp.AlertCamp` _assignedcamp self (`self.TargetActor`)))
    (:`else`)))

(fn `SetWeaponOwner`
  (bind _childactor (`ChildActorComponent.ChildActor` (`self.WeaponActorComponent`))
    (:`then`
      (`self.SetOwner` _childactor self))
    (:`else`)))

(fn `UserConstructionScript`
  (`self.SetWeaponOwner`)
  (`self.CreateDynamicMaterialInstance`))