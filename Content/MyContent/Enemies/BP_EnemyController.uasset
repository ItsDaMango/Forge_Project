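; AI controller for BP_Enemy that runs the pawn's behavior tree on possession and stops it on death.
; AI Perception locks onto the first living player sensed while no target is set, writing it to the Blackboard and enemy.
; PickPlayerToAttack caches nearby players and targets the closer living one of two, falling back to the passed actor.
; Blackboard keys also carry attack range and interrupt duration to the tree.
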(event `self.ReceivePossess`
  (params (PossessedPawn :type "Pawn Object Reference"))
  (bind _asbp_enemy (cast `/Game/MyContent/Enemies/BP_Enemy` PossessedPawn))
  (bind _output_get (set `self.EnemyRef` _asbp_enemy))
  (add `/Game/MyContent/Enemies/BP_Enemy.OnDeath` _asbp_enemy (`|CreateDelegate` :!event `OnDeath`))
  (bind _behaviour (`/Game/MyContent/Enemies/BP_Enemy.Behaviour` _output_get)
    (:`then`
      (`self.RunBehaviorTree` _behaviour)
      (`self.SetDefaultBBKeys`))
    (:`else`)))

(event `self.AIPerception.OnTargetPerceptionUpdated`
  (params (Actor :type "Actor Object Reference") (Stimulus :type "AIStimulus Structure"))
  (if (not (`KismetSystemLibrary.IsValid` (`self.TargetActor`)))
    (bind _asbp_player_character (cast `/Game/MyContent/Player/BP_PlayerCharacter` Actor))
    (if (`/Game/MyContent/Core/BP_AC_Stats.IsAlive` (`/Game/MyContent/Player/BP_PlayerCharacter.StatComponent` _asbp_player_character))
      (`self.SetControlTarget` _asbp_player_character))))

(event `ResetPerception`
  (`AIPerceptionComponent.ForgetAll` (`self.AIPerception`)))

(event `OnDeath`
  (`BrainComponent.StopLogic` (`self.BrainComponent`) "Died"))

(fn `InteruptAI`
  (params (Duration :type "Float (single-precision)"))
  (`BlackboardComponent.SetValueAsFloat` (`AIBlueprintHelperLibrary.GetBlackboard` null) "InteruptTime" Duration))

(fn `PickPlayerToAttack`
  (params (Actor :type "Actor Object Reference"))
  (returns (`Failed Abort` :type Boolean))
  (bind _returnvalue (`self.K2_GetPawn`))
  (bind _players (`self.Players`))
  (bind _output (`|GetArrayItem` (`self.Players`) 1))
  (bind _output_2 (`|GetArrayItem` (`self.Players`)))
  (bind _output_3 (`|GetArrayItem` (`self.Players`) 1))
  (bind _output_4 (`|GetArrayItem` (`self.Players`)))
  (if (`KismetArrayLibrary.Array_IsEmpty` (`self.Players`))
    (bind (_outactors _returnvalue_2) (`KismetSystemLibrary.SphereOverlapActors` (`self.K2_GetActorLocation` (`self.K2_GetPawn`)) 1000.0 (`|MakeArray` "ObjectTypeQuery3" :!type "EObjectTypeQuery Enum") "/Game/MyContent/Player/BP_PlayerCharacter.BP_PlayerCharacter_C" (`|MakeArray` self :!type "Actor Object Reference")))
    (if (and _returnvalue_2 (> (`KismetArrayLibrary.Array_Length` _outactors) 1))
      (for _array_element _outactors
        (bind _asbp_player_character (cast `/Game/MyContent/Player/BP_PlayerCharacter` _array_element))
        (`KismetArrayLibrary.Array_Add` (`self.Players`) _asbp_player_character))
      (else
        (bind _asbp_player_character_2 (cast `/Game/MyContent/Player/BP_PlayerCharacter` (`local.Actor`) :!label _label))
        (if (`/Game/MyContent/Core/BP_AC_Stats.IsAlive` (`/Game/MyContent/Player/BP_PlayerCharacter.StatComponent` _asbp_player_character_2))
          (`self.SetControlTarget` _asbp_player_character_2)
          (`KismetSystemLibrary.PrintString` "only 1 player in range / Default First Pick" true true (struct :`R` 0.001826 :`B` 1.0 :`A` 1.0))
          (return false)
          (else
            (`self.SetControlTarget` null)
            (`KismetSystemLibrary.PrintString` "only 1 player in range. And they are dead / Default Fail" true true (struct :`R` 0.002568 :`B` 1.0 :`A` 1.0))
            (return true)))))
    (elif (> (`KismetArrayLibrary.Array_Length` (`self.Players`)) 1)
      _
      (else
        (goto _label))))
  (if (< (`self.GetDistanceTo` (`|GetArrayItem` _players) _returnvalue) (`self.GetDistanceTo` (`|GetArrayItem` _players 1) _returnvalue))
    (if (`/Game/MyContent/Core/BP_AC_Stats.IsAlive` (`/Game/MyContent/Player/BP_PlayerCharacter.StatComponent` _output_4))
      (`self.SetControlTarget` _output_4)
      (`KismetSystemLibrary.PrintString` "P1 Focus")
      (elif (`/Game/MyContent/Core/BP_AC_Stats.IsAlive` (`/Game/MyContent/Player/BP_PlayerCharacter.StatComponent` _output))
        (`self.SetControlTarget` _output)
        (`KismetSystemLibrary.PrintString` "P1 Dead, Focus  \nP2" true true (struct :`G` 1.0 :`B` 0.18893 :`A` 1.0))
        (return false)
        (else
          (`self.SetControlTarget` null)
          (`KismetSystemLibrary.PrintString` "Both dead" true true (struct :`R` 1.0 :`B` 0.054088 :`A` 1.0))
          (return true))))
    (elif (`/Game/MyContent/Core/BP_AC_Stats.IsAlive` (`/Game/MyContent/Player/BP_PlayerCharacter.StatComponent` _output_3))
      (`self.SetControlTarget` _output_3)
      (`KismetSystemLibrary.PrintString` "P2 Focus")
      (elif (`/Game/MyContent/Core/BP_AC_Stats.IsAlive` (`/Game/MyContent/Player/BP_PlayerCharacter.StatComponent` _output_2))
        (`self.SetControlTarget` _output_2)
        (`KismetSystemLibrary.PrintString` "P2 Dead, Focus  \nP1" true true (struct :`G` 1.0 :`B` 0.114498 :`A` 1.0))
        (return false)
        (else
          (`self.SetControlTarget` null)
          (`KismetSystemLibrary.PrintString` "Both dead" true true (struct :`R` 1.0 :`B` 0.054088 :`A` 1.0))
          (return true))))))

(fn `SetControlTarget`
  (params (Actor :type "Actor Object Reference"))
  (bind _output_get (set `self.TargetActor` Actor))
  (`BlackboardComponent.SetValueAsObject` (`AIBlueprintHelperLibrary.GetBlackboard` null) "TargetActor" _output_get)
  (`/Game/MyContent/Enemies/BP_Enemy.SetEnemyTarget` (`self.EnemyRef`) (`self.TargetActor`)))

(fn `SetDefaultBBKeys`
  (`BlackboardComponent.SetValueAsFloat` (`AIBlueprintHelperLibrary.GetBlackboard` null) "AttackRange" (`/Game/MyContent/Enemies/BP_Enemy.AttackRange` (`self.EnemyRef`))))

(fn `UserConstructionScript`)